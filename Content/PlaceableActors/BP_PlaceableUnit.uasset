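; Placeable turret unit with a cost, which tracks and shoots actors tagged "Ennemy" or "Targetable" entering its Range.
; Overlaps set or release the target lock, and Tick switches between yaw-only tracking with firing and an idle spin.
; A Delay called from Tick throttles projectile spawns at the Canon_Socket; the FireRate calculation is unconnected.
; Construction script applies the meshes, while static mesh rotation is marked as a placeholder until an animated mesh is used.
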(event `self.ReceiveBeginPlay`
  (set `self.Cost` (`self.Cost`)))

(event `self.Range.OnComponentBeginOverlap`
  (params (OverlappedComponent :type "PrimitiveComponent Object Reference") (OtherActor :type "Actor Object Reference") (OtherComp :type "PrimitiveComponent Object Reference") (OtherBodyIndex :type Integer) (bFromSweep :type Boolean) (SweepResult :type "HitResult Structure (by ref)"))
  (if (or (`self.ActorHasTag` OtherActor "Ennemy") (`self.ActorHasTag` OtherActor "Targetable"))
    (set `self.Target` OtherActor)
    (set `self.bLockedTarget` true)
    (`KismetSystemLibrary.PrintString` "Should fire")))

(event `self.Range.OnComponentEndOverlap`
  (params (OverlappedComponent :type "PrimitiveComponent Object Reference") (OtherActor :type "Actor Object Reference") (OtherComp :type "PrimitiveComponent Object Reference") (OtherBodyIndex :type Integer))
  (set `self.bLockedTarget` false))

(event `self.ReceiveTick`
  (params (DeltaSeconds :type "Float (single-precision)"))
  (if (`self.bLockedTarget`)
    (`self.UpdateTurretRotation`)
    (`self.Firing`)
    (else
      (`self.Turret Idle`))))

(event `UpdateTurretRotation`
  (`SceneComponent.K2_SetWorldRotation` (`self.Mesh`) (`self.TurretRotation`) false false))

(event `Turret Idle`
  (`SceneComponent.K2_SetWorldRotation` (`self.Mesh`) (`self.TurretIDLE`) false false))

(event `Firing`
  (`KismetSystemLibrary.Delay` 0.2)
  (`|SpawnActorFromClass` (`self.ProjectileClass`) (`SceneComponent.GetSocketTransform` (`self.Mesh`) "Canon_Socket" "RTS_World") "Undefined" "OverrideRootScale" null null))

(fn `UserConstructionScript`
  ;[1 0 0] DEBUG VISUALIZATION
  (`StaticMeshComponent.SetStaticMesh` (`self.Mesh`) (`self.TurretMesh`))
  (`SkinnedMeshComponent.SetSkinnedAssetAndUpdate` (`self.Turret`) (`self.SKEL_TurretMesh`) true)
  (set `self.ProjectileClass` (`self.ProjectileClass`)))