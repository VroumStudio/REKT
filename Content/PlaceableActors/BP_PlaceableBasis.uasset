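; BP_PlaceableBasis is a pedestal actor that marks a spot for a placeable turret, though it spawns nothing itself.
; On BeginPlay it disables Custom Depth and stores a dynamic pedestal material.
; The first cursor hover enables Custom Depth, stores and prints a spawn transform above the mesh, and sets SpawnedTurret, blocking later highlights.
; Cursor exit clears Custom Depth; a disconnected AddToViewport branch never runs.
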(event `self.ReceiveBeginPlay`
  (`PrimitiveComponent.SetRenderCustomDepth` (`self.StaticMeshComponent`) false)
  (bind _returnvalue (`PrimitiveComponent.CreateDynamicMaterialInstance` (`self.StaticMeshComponent`) 0 "/Game/PlaceableActors/Turret_Pedestal/BL_Pedestal.BL_Pedestal" "None"))
  (set `self.DMI_Pedestral` _returnvalue))

(event `self.StaticMeshComponent.OnBeginCursorOver`
  (params (TouchedComponent :type "PrimitiveComponent Object Reference"))
  (if (not (`self.bSpawnedTurret`))
    (`PrimitiveComponent.SetRenderCustomDepth` (`self.StaticMeshComponent`) true)
    (bind _output_get (set `self.PlaceableUnitSpawnPoint` (`KismetMathLibrary.MakeTransform` (+ (`SceneComponent.K2_GetComponentLocation` (`self.StaticMeshComponent`)) (0.0 0.0 50.0)))))
    (`KismetSystemLibrary.PrintString` (`KismetStringLibrary.Conv_TransformToString` _output_get))
    (set `self.bSpawnedTurret` true)))

(event `self.StaticMeshComponent.OnEndCursorOver`
  (params (TouchedComponent :type "PrimitiveComponent Object Reference"))
  (`PrimitiveComponent.SetRenderCustomDepth` (`self.StaticMeshComponent`) false))

(fn `UserConstructionScript`)