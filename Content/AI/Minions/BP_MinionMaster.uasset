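; BP_MinionMaster is a minion AI actor, apparently a shared base, still at an early stage.
; On BeginPlay it caches the player's BP_MasterVehicle and, if that cast succeeds, the first BP_PatrolPath in the level.
; Tick only prints the patrol path's name as debug output.
; The capsule overlap checks for a Vehicle tag but does nothing, and logic to reduce the vehicle body's velocity is left unconnected.
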(event `self.ReceiveBeginPlay`
  (bind _asbp_master_vehicle (cast `/Game/Vehicles/MasterVehicle/BP_MasterVehicle` (`GameplayStatics.GetPlayerPawn` 0)))
  (set `self.BPREF_MasterVehicle` _asbp_master_vehicle)
  (bind _outactors (`GameplayStatics.GetAllActorsOfClass` "/Game/AI/BP_PatrolPath.BP_PatrolPath_C"))
  (set `self.PatrolPath` (`|GetArrayItem` _outactors)))

(event `self.ReceiveTick`
  (params (DeltaSeconds :type "Float (single-precision)"))
  (`KismetSystemLibrary.PrintString` (`KismetSystemLibrary.GetDisplayName` (`self.PatrolPath`)) true true (struct :`G` 0.66 :`B` 1.0 :`A` 1.0) 0.0))

(event `self.CapsuleComponent.OnComponentBeginOverlap`
  (params (OverlappedComponent :type "PrimitiveComponent Object Reference") (OtherActor :type "Actor Object Reference") (OtherComp :type "PrimitiveComponent Object Reference") (OtherBodyIndex :type Integer) (bFromSweep :type Boolean) (SweepResult :type "HitResult Structure (by ref)"))
  (if (`self.ActorHasTag` OtherActor "Vehicle")
    _))

(fn `UserConstructionScript`)