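; BP_EnnemiesSpawner is a trigger actor that spawns a group of AI enemies when an actor tagged "Vehicle" enters its Box.
; The overlap event loops on Type01Quantity, spawning BP_MasterEnemy pawns that run the BT_Minion behavior tree.
; Each spawn takes the Arrow component's height and rotation, with a random horizontal offset around it.
; Nothing disables the trigger, so every qualifying overlap spawns another group.
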(event `self.Box.OnComponentBeginOverlap`
  (params (OverlappedComponent :type "PrimitiveComponent Object Reference") (OtherActor :type "Actor Object Reference") (OtherComp :type "PrimitiveComponent Object Reference") (OtherBodyIndex :type Integer) (bFromSweep :type Boolean) (SweepResult :type "HitResult Structure (by ref)"))
  (bind _returnvalue (`KismetMathLibrary.RandomFloatInRange` -500.0 500.0))
  (bind _returnvalue_2 (`SceneComponent.K2_GetComponentToWorld` (`self.Arrow`)))
  (if (`self.ActorHasTag` OtherActor "Vehicle")
    (`|ExecutionSequence`
      (:`then_0`
        (for _ (range (+ (`self.Type01Quantity`) 1))
          (`AIBlueprintHelperLibrary.SpawnAIFromClass` "/Game/AI/BP_MasterEnemy.BP_MasterEnemy_C" "/Game/AI/Minions/BT_Minion.BT_Minion" (`KismetMathLibrary.MakeVector` (+ (.x (.location _returnvalue_2)) _returnvalue) (+ (.y (.location _returnvalue_2)) _returnvalue) (.z (.location _returnvalue_2))) (.rotation _returnvalue_2)))))))

(fn `UserConstructionScript`)