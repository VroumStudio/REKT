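; Base enemy Blueprint that handles damage, death and player rewards.
; On BeginPlay it caches the player pawn as a BP_MasterVehicle.
; Incoming damage is reduced by flat Armor, then subtracted from Health or triggers death if lethal.
; Death adds score and currency to the vehicle, decrements its remaining-enemy count, destroys the actor and spawns explosion and money-drop particles.
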(event `self.ReceiveBeginPlay`
  (bind _asbp_master_vehicle (cast `/Game/Vehicles/MasterVehicle/BP_MasterVehicle` (`GameplayStatics.GetPlayerPawn` 0)))
  (set `self.BPREF_MasterVehicle` _asbp_master_vehicle))

(event `self.ReceiveAnyDamage`
  (params (Damage :type "Float (single-precision)") (DamageType :type "DamageType Object Reference") (InstigatedBy :type "Controller Object Reference") (DamageCauser :type "Actor Object Reference"))
  (bind _returnvalue (- (`self.Health`) (- Damage (`self.Armor`))))
  (if (<= _returnvalue 0.0)
    (`self.EVNT_Death`)
    (else
      (set `self.Health` _returnvalue))))

(event `EVNT_Death`
  (bind _bpref_mastervehicle (`self.BPREF_MasterVehicle`))
  (set `/Game/Vehicles/MasterVehicle/BP_MasterVehicle.Score` (+ (`/Game/Vehicles/MasterVehicle/BP_MasterVehicle.Score` _bpref_mastervehicle) (`self.ScoreGiven`)) _bpref_mastervehicle)
  (set `/Game/Vehicles/MasterVehicle/BP_MasterVehicle.Currency` (+ (`/Game/Vehicles/MasterVehicle/BP_MasterVehicle.Currency` _bpref_mastervehicle) (`self.CurrencyGiven`)) _bpref_mastervehicle)
  (set `/Game/Vehicles/MasterVehicle/BP_MasterVehicle.RemainingEnemies` (- (`/Game/Vehicles/MasterVehicle/BP_MasterVehicle.RemainingEnemies` _bpref_mastervehicle) 1) _bpref_mastervehicle)
  (`self.K2_DestroyActor`)
  (`GameplayStatics.SpawnEmitterAtLocation` "/Game/FX/Minion_Explosion/PS_Minion_Explosion.PS_Minion_Explosion" (`self.K2_GetActorLocation`))
  (`GameplayStatics.SpawnEmitterAtLocation` "/Game/FX/FX_Money_Drop/PS_Money_Drop.PS_Money_Drop" (`self.K2_GetActorLocation`)))

(fn `UserConstructionScript`)