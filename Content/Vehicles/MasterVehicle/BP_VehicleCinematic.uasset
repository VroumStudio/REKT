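; BP_VehicleCinematic is a physics-constraint vehicle whose construction script builds wheels and suspension for a configurable number of axles.
; SetAxle syncs the axle settings array to the axle count, then each axle spawns two mirrored skeletal-mesh wheels with spring-driven vertical constraints.
; Axles at X >= 1 link wheels to a fake suspension rod mesh, which a steering constraint joins to the Body; other wheels constrain directly to the Body.
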(fn `SetAxle`
  (bind _axle (`self.Axle`))
  (bind _s_axle (`self.S_Axle`))
  (bind _s_axle_2 (`self.S_Axle`))
  (bind _returnvalue (`KismetArrayLibrary.Array_Length` _s_axle))
  (if (< _returnvalue _axle) :!label _label
    (`KismetArrayLibrary.Array_Add` _s_axle_2 (`self.Axle_Defaults`))
    (goto _label)
    (elif (> _returnvalue _axle)
      (`KismetArrayLibrary.Array_Remove` _s_axle_2 (`KismetArrayLibrary.Array_LastIndex` _s_axle))
      (goto _label)
      (else
        (set `self.TotalWheels` (* _axle 2))))))

(fn `UserConstructionScript`
  (`self.SetAxle`)
  (for _index (range (`self.Axle`))
    (for _index_2 (range 2)
      (bind (_position _radius _applytorque _brakestrengthmultiplier _suspensionlength _suspensionstrength _suspensiondamping _wheelmesh) (break `/Game/Vehicles/MasterVehicle/Setup/Structures/S_Axle` (`|GetArrayItem` (`self.S_Axle`) _index)))
      (bind _returnvalue (`KismetMathLibrary.MakeTransform` (`KismetMathLibrary.MakeVector` (.x _position) (* (.y _position) (select `int` _index_2 :`0` -1.0 :`1` 1.0 :!type "Float (single-precision)")) (.z _position)) (struct) (`KismetMathLibrary.MakeVector` 1.0 (select `int` _index_2 :`0` -1.0 :`1` 1.0 :!type "Float (single-precision)") 1.0)))
      (bind _returnvalue_2 (`AddComponent|NODE_AddPhysicsConstraintComponent-2` :`RelativeTransform` _returnvalue)) ; Suspension & Roll Handling
      (`KismetArrayLibrary.Array_Add` (`self.AxleConstraints`) _returnvalue_2)
      (if (>= (.x _position) 1.0)
        (bind _returnvalue_3 (`KismetMathLibrary.MakeTransform` (`KismetMathLibrary.MakeVector` (.x _position) (* (.y _position) (select `int` _index_2 :`0` -1.0 :`1` 1.0 :!type "Float (single-precision)")) (.z _position)) (struct) (1.0 1.0 1.0)))
        (bind _returnvalue_4 (`AddComponent|NODE_AddStaticMeshComponent-1` :`RelativeTransform` _returnvalue_3)) ; 'Fake' suspension rod mesh
        (bind _returnvalue_5 (`AddComponent|NODE_AddSkeletalMeshComponent-0` :`RelativeTransform` _returnvalue))
        (`SkinnedMeshComponent.SetSkinnedAssetAndUpdate` _returnvalue_5 _wheelmesh false)
        (`SkinnedMeshComponent.SetPhysicsAsset` _returnvalue_5 (`SkeletalMesh.PhysicsAsset` _wheelmesh) false)
        (`KismetArrayLibrary.Array_Add` (`self.WheelsMeshes`) _returnvalue_5)
        (`PhysicsConstraintComponent.SetConstrainedComponents` _returnvalue_2 _returnvalue_5 "None" _returnvalue_4 "None")
        (`PhysicsConstraintComponent.SetLinearZLimit` _returnvalue_2 "LCM_Limited" _suspensionlength)
        (`PhysicsConstraintComponent.SetLinearDriveParams` _returnvalue_2 _suspensionstrength _suspensiondamping 0.0)
        (`PhysicsConstraintComponent.SetLinearPositionTarget` _returnvalue_2 (`KismetMathLibrary.MakeVector` 0.0 0.0 (* _suspensionlength -0.5)))
        (bind _returnvalue_6 (`AddComponent|NODE_AddPhysicsConstraintComponent-3` :`RelativeTransform` _returnvalue_3)) ; Steering Constraints
        (`PhysicsConstraintComponent.SetConstrainedComponents` _returnvalue_6 (`self.Body`) "None" _returnvalue_4 "None")
        (`KismetArrayLibrary.Array_Add` (`self.SteeringConstraints`) _returnvalue_6)
        (else
          (bind _returnvalue_7 (`AddComponent|NODE_AddSkeletalMeshComponent-1` :`RelativeTransform` _returnvalue))
          (`SkinnedMeshComponent.SetSkinnedAssetAndUpdate` _returnvalue_7 _wheelmesh false)
          (`SkinnedMeshComponent.SetPhysicsAsset` _returnvalue_7 (`SkeletalMesh.PhysicsAsset` _wheelmesh) false)
          (`KismetArrayLibrary.Array_Add` (`self.WheelsMeshes`) _returnvalue_7)
          (`PhysicsConstraintComponent.SetConstrainedComponents` _returnvalue_2 _returnvalue_7 "None" (`self.Body`) "None")
          (`PhysicsConstraintComponent.SetLinearZLimit` _returnvalue_2 "LCM_Limited" _suspensionlength)
          (`PhysicsConstraintComponent.SetLinearDriveParams` _returnvalue_2 _suspensionstrength _suspensiondamping 0.0)
          (`PhysicsConstraintComponent.SetLinearPositionTarget` _returnvalue_2 (`KismetMathLibrary.MakeVector` 0.0 0.0 (* _suspensionlength -0.5))))))))