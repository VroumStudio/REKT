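; Drivable muscle car Blueprint with custom raycast vehicle physics on a physics chassis.
; Each tick, four wheel traces drive spring-damper suspension, whose load scales throttle-based longitudinal and slip-velocity lateral tire forces applied to the chassis.
; Input handles steering, camera, an engine RPM/torque simulation and delayed gear shifts through neutral; engine and gear outputs don't yet feed tire forces.
; Includes debug prints, force lines and a reset key.
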(event `self.ReceiveBeginPlay`
  (`self.ArrayInitialization`)
  (`self.Initialization`)
  (`self.GetUnitConvertMult`))

(event `self.ReceiveTick`
  (params (DeltaSeconds :type "Float (single-precision)"))
  (set `self.DeltaSeconds` DeltaSeconds)
  (`self.WheelsRayCast`)
  (`self.UpdateSuspensionsLength`)
  (`self.GetSuspensionForce`)
  (`self.ApplySuspensionForce`)
  (`self.UpdateWheelLocation`)
  (`self.GetWheelLinearVelocityLocal`)
  (`self.GetTireForces`)
  (`self.ApplyTireForces`)
  (`self.WheelRotation`)
  (`self.DisplayDebugForces`)
  (`self.RandomizeIDLEEngineRPM`)
  (`KismetSystemLibrary.PrintString` (`KismetStringLibrary.Concat_StrStr` "Gear: " (select `int` (`self.Gear`) :`0` "R" :`1` "N" :`2` "1" :`3` "2" :`4` "3" :`5` "4" :`6` "5" :`7` "6")) true true (struct :`G` 0.4 :`A` 1.0) 0.0))

(event `InputAxis|LookUp`
  (params (AxisValue :type "Float (single-precision)"))
  (`self.LookAround` :!label _label))

(event `InputAxis|LookRight`
  (params (AxisValue :type "Float (single-precision)"))
  (goto _label))

(event `InputAxis|Throttle`
  (params (AxisValue :type "Float (single-precision)"))
  (`self.GetThrottleValue` AxisValue)
  (`self.GetEngineTorque`))

(event `InputAxis|SteerRight`
  (params (AxisValue :type "Float (single-precision)"))
  (`self.SetSteeringInput` AxisValue))

(event `Key|Tab`
  (params (Key :type "Key Structure"))
  (bind _chassis_mesh (`self.Chassis_Mesh`))
  ;[0.3 0 0] Enter/Exit debug mode (DEBUG ONLY)
  (:`Pressed`
    (`/Engine/EditorBlueprintResources/StandardMacros.FlipFlop`
      (:`A`
        (set `self.bDisplayDebugForces` true)
        (`SceneComponent.SetVisibility` _chassis_mesh false false))
      (:`B`
        (set `self.bDisplayDebugForces` false)
        (`SceneComponent.SetVisibility` _chassis_mesh true false)))))

(event `Key|R`
  (params (Key :type "Key Structure"))
  (bind _chassis_mesh (`self.Chassis_Mesh`))
  (bind _returnvalue (`SceneComponent.K2_GetComponentToWorld` _chassis_mesh))
  ;[0.3 0 0] Respawn car (DEBUG ONLY)
  (:`Pressed`
    (`SceneComponent.K2_SetWorldTransform` _chassis_mesh (`KismetMathLibrary.MakeTransform` (+ (.location _returnvalue) (0.0 0.0 100.0)) (`KismetMathLibrary.MakeRotator` 0.0 0.0 (.yaw (.rotation _returnvalue)))) false true)))

(event `InputAction|GearUp`
  (params (Key :type "Key Structure"))
  (:`Pressed`
    (set `self.GearTarget` (`KismetMathLibrary.Min` (+ (`self.Gear`) 1) (- (`KismetArrayLibrary.Array_Length` (`self.GearRatio`)) 1)))
    (set `self.Gear` 1)
    (set `self.TotalGearRatio` 0.0)
    (`KismetSystemLibrary.Delay` (`self.GearChangeTime`))
    (bind _output_get (set `self.Gear` (`self.GearTarget`)))
    (set `self.TotalGearRatio` (* (`|GetArrayItem` (`self.GearRatio`) _output_get) (`self.MainGear`)))))

(event `InputAction|GearDown`
  (params (Key :type "Key Structure"))
  (:`Pressed`
    (set `self.GearTarget` (`KismetMathLibrary.Max` (- (`self.Gear`) 1)))
    (set `self.Gear` 1)
    (set `self.TotalGearRatio` 0.0)
    (`KismetSystemLibrary.Delay` (`self.GearChangeTime`))
    (bind _output_get (set `self.Gear` (`self.GearTarget`)))
    (set `self.TotalGearRatio` (* (`|GetArrayItem` (`self.GearRatio`) _output_get) (`self.MainGear`)))))

(fn `ApplySuspensionForce`
  (for _index (range 4)
    (bind _output (`|GetArrayItem` (`self.TopLinkComponent`) _index))
    (`PrimitiveComponent.AddForceAtLocation` (`self.Chassis_Mesh`) (* (`SceneComponent.GetUpVector` _output) (* (`|GetArrayItem` (`self.Fz`) _index) 100.0)) (`SceneComponent.K2_GetComponentLocation` _output) "None")))

(fn `ApplyTireForces`
  (for _index (range 4)
    (if (`|GetArrayItem` (`self.bWheelContact`) _index)
      (bind _output (`|GetArrayItem` (`self.TopLinkComponent`) _index))
      (`PrimitiveComponent.AddForceAtLocation` (`self.Chassis_Mesh`) (* (+ (* (`SceneComponent.GetForwardVector` _output) (`|GetArrayItem` (`self.Fx`) _index)) (* (`SceneComponent.GetRightVector` _output) (`|GetArrayItem` (`self.Fy`) _index))) 100.0) (`.Location` (`GameplayStatics.BreakHitResult` (`|GetArrayItem` (`self.HitResult`) _index))) "None"))))

(fn `ArrayInitialization`
  (for _index (range 4)
    (`KismetArrayLibrary.Array_Set` (`self.TopLinkComponent`) _index (select `int` _index :`0` (`self.TopLink_FL`) :`1` (`self.TopLink_FR`) :`2` (`self.TopLink_RL`) :`3` (`self.TopLink_RR`)))
    (`KismetArrayLibrary.Array_Set` (`self.WheelComponent`) _index (select `int` _index :`0` (`self.Wheel_FL`) :`1` (`self.Wheel_FR`) :`2` (`self.Wheel_RL`) :`3` (`self.Wheel_RR`) :!type "SceneComponent Object Reference"))))

(fn `DisplayDebugForces`
  (if (`self.bDisplayDebugForces`)
    (for _index (range 4)
      (for _index_2 (range 3)
        (bind _returnvalue (`SceneComponent.K2_GetComponentLocation` (`|GetArrayItem` (`self.WheelComponent`) _index)))
        (bind _output (`|GetArrayItem` (`self.TopLinkComponent`) _index))
        (`KismetSystemLibrary.DrawDebugLine` _returnvalue (+ _returnvalue (* (select `int` _index_2 :`0` (`SceneComponent.GetForwardVector` _output) :`1` (`SceneComponent.GetRightVector` _output) :`2` (`SceneComponent.GetUpVector` _output)) (/ (select `int` _index_2 :`0` (`|GetArrayItem` (`self.Fx`) _index) :`1` (`|GetArrayItem` (`self.Fy`) _index) :`2` (`|GetArrayItem` (`self.Fz`) _index)) 40.0))) (select `int` _index_2 :`0` (struct :`R` 1.0 :`A` 1.0) :`1` (struct :`G` 1.0 :`A` 1.0) :`2` (struct :`B` 1.0 :`A` 1.0) :!type "LinearColor Structure") 0.0 8.0)))))

(fn `GetEngineTorque`
  (bind _throttlevalue (`self.ThrottleValue`))
  (bind _rpmtoradiansps (`self.RPMToRadiansPS`))
  (bind (_torquecurve _rpmidle _rpmmax) (break `/Game/Vehicles/MuscleCarV2/Setup/Structures/S_Engine` (`self.Engine`)))
  (bind (_torquecurve_2 _rpmidle_2 _rpmmax_2 _inertia _backtorque) (break `/Game/Vehicles/MuscleCarV2/Setup/Structures/S_Engine` (`self.Engine`)))
  ;[1 1 1] AngularAcceleration=Torque/Inertia
  (bind _output_get (set `self.EngineTorque` (`KismetMathLibrary.Lerp` _backtorque (* (`CurveFloat.GetFloatValue` _torquecurve_2 (`self.EngineRPM`)) _throttlevalue) _throttlevalue)))
  (bind _output_get_2 (set `self.EngineAngularVelocity` (`KismetMathLibrary.FClamp` (+ (`self.EngineAngularVelocity`) (* (/ _output_get _inertia) (`self.DeltaSeconds`))) (* _rpmtoradiansps _rpmidle) (* _rpmtoradiansps _rpmmax))))
  (bind _output_get_3 (set `self.EngineRPM` (* _output_get_2 (`self.RadiansPSToRPM`))))
  (`KismetSystemLibrary.PrintString` (`KismetStringLibrary.Concat_StrStr` "Engine RPM: " (`KismetStringLibrary.Conv_DoubleToString` _output_get_3)) true true (struct :`R` 1.0 :`B` 0.2 :`A` 1.0) 0.0)
  (`KismetSystemLibrary.PrintString` (`KismetStringLibrary.Concat_StrStr` "Engine Torque: " (`KismetStringLibrary.Conv_DoubleToString` (`self.EngineTorque`))) true true (struct :`R` 1.0 :`B` 0.2 :`A` 1.0) 0.0))

(fn `GetSuspensionForce`
  (for _index (range 4)
    (bind (_namedebugonly _restlength _travel _stiffness _damper _minforce _maxforce) (break `/Game/Vehicles/MuscleCarV2/Setup/Structures/S_Suspension` (`|GetArrayItem` (`self.Suspension`) _index)))
    (bind _output (`|GetArrayItem` (`self.Length`) _index))
    (bind _returnvalue (`KismetMathLibrary.FClamp` (+ (* (- _restlength _output) _stiffness) (* _damper (/ (- (`|GetArrayItem` (`self.PreviousLength`) _index) _output) (`self.DeltaSeconds`)))) _minforce _maxforce))
    (`KismetArrayLibrary.Array_Set` (`self.Fz`) _index _returnvalue)
    (`KismetArrayLibrary.Array_Set` (`self.PreviousLength`) _index (`|GetArrayItem` (`self.Length`) _index))
    (`KismetSystemLibrary.PrintString` (`KismetStringLibrary.Concat_StrStr` (select `int` _index :`0` "Fz_FL: " :`1` "Fz_RL: " :`2` "Fz_RR: " :`3` "Fz_FR: ") (`KismetStringLibrary.Conv_DoubleToString` _returnvalue)) true true (struct :`B` 1.0 :`A` 1.0) 0.0)))

(fn `GetThrottleValue`
  (params (InputPin :type "Float (double-precision)"))
  (bind _throttlevalue (`self.ThrottleValue`))
  (bind _deltaseconds (`self.DeltaSeconds`))
  (if (`self.ThrottleFilter`)
    (if (!= InputPin 0.0)
      (set `self.ThrottleValue` (`KismetMathLibrary.FMin` (+ _throttlevalue (* _deltaseconds 1.0)) 1.0))
      (else
        (set `self.ThrottleValue` (`KismetMathLibrary.FMax` (- _throttlevalue (* _deltaseconds 2.0))))))
    (else
      (set `self.ThrottleValue` InputPin)))
  (`KismetSystemLibrary.PrintString` (`KismetStringLibrary.Concat_StrStr` "Throttle Value: " (`KismetStringLibrary.Conv_DoubleToString` (`self.ThrottleValue`))) true true (struct :`R` 1.0 :`G` 0.125 :`A` 1.0) 0.0))

(fn `GetTireForces`
  (for _index (range 4)
    (if (`|GetArrayItem` (`self.bWheelContact`) _index)
      (bind _output (`|GetArrayItem` (`self.Fz`) _index))
      (`KismetArrayLibrary.Array_Set` (`self.Fx`) _index (* (`self.GetInputAxisValue`) _output 0.5))
      (bind (_output_x _output_y) (`KismetMathLibrary.BreakVector` (`|GetArrayItem` (`self.WheelLinearVelocityLocal`) _index)))
      (`KismetArrayLibrary.Array_Set` (`self.Fy`) _index (`KismetMathLibrary.FClamp` (* _output _output_y -1.0) (* _output -1.0) _output))
      (else
        (`KismetArrayLibrary.Array_Set` (`self.Fx`) _index)
        (`KismetArrayLibrary.Array_Set` (`self.Fy`) _index)))))

(fn `GetUnitConvertMult`
  (bind _output_get (set `self.RPMToRadiansPS` (/ 60.0 (* (`KismetMathLibrary.GetPI`) 2.0))))
  (set `self.RadiansPSToRPM` (/ 1.0 _output_get)))

(fn `GetWheelLinearVelocityLocal`
  (for _index (range 4)
    (bind _output (`|GetArrayItem` (`self.TopLinkComponent`) _index))
    (bind _returnvalue (`PrimitiveComponent.GetPhysicsLinearVelocityAtPoint` (`self.Chassis_Mesh`) (- (`SceneComponent.K2_GetComponentLocation` (`|GetArrayItem` (`self.WheelComponent`) _index)) (* (`SceneComponent.GetUpVector` _output) (`.Radius_2_31E569DA423D4B98C93673A340DDDC2B` (break `/Game/Vehicles/MuscleCarV2/Setup/Structures/S_Wheel` (`|GetArrayItem` (`self.Wheel`) _index))))) "None"))
    (bind _returnvalue_2 (`KismetMathLibrary.TransformDirection` (`KismetMathLibrary.InvertTransform` (`SceneComponent.K2_GetComponentToWorld` _output)) (/ _returnvalue 100.0)))
    (`KismetArrayLibrary.Array_Set` (`self.WheelLinearVelocityLocal`) _index _returnvalue_2)
    (`KismetSystemLibrary.PrintString` (`KismetStringLibrary.Conv_VectorToString` _returnvalue_2) true true (struct :`G` 0.66 :`B` 1.0 :`A` 1.0) 0.0)))

(fn `Initialization`
  (for _index (range 4)
    (bind ((`RestLength_2_31E569DA423D4B98C93673A340DDDC2B` _restlength) (`Travel_11_5C5EEE8B4B37DC4C427D1EA14FB77726` _travel)) (break `/Game/Vehicles/MuscleCarV2/Setup/Structures/S_Suspension` (`|GetArrayItem` (`self.Suspension`) _index)))
    (`KismetArrayLibrary.Array_Set` (`self.RayLength`) _index (+ (+ _restlength _travel) (`.Radius_2_31E569DA423D4B98C93673A340DDDC2B` (break `/Game/Vehicles/MuscleCarV2/Setup/Structures/S_Wheel` (`|GetArrayItem` (`self.Wheel`) _index)))))
    (bind (_namedebugonly _restlength_2) (break `/Game/Vehicles/MuscleCarV2/Setup/Structures/S_Suspension` (`|GetArrayItem` (`self.Suspension`) _index)))
    (`KismetArrayLibrary.Array_Set` (`self.Length`) _index _restlength_2)
    (`KismetArrayLibrary.Array_Set` (`self.PreviousLength`) _index _restlength_2)))

(fn `LookAround`
  (bind _followcamspringarm (`self.FollowCamSpringArm`))
  (bind (_relativerotation_roll _relativerotation_pitch _relativerotation_yaw) (`KismetMathLibrary.BreakRotator` (`SceneComponent.RelativeRotation` _followcamspringarm)))
  (`SceneComponent.K2_AddRelativeRotation` _followcamspringarm (`KismetMathLibrary.MakeRotator` 0.0 (`self.GetInputAxisValue`) (`self.GetInputAxisValue`)) false false)
  (`SceneComponent.K2_SetRelativeRotation` _followcamspringarm (`KismetMathLibrary.SelectRotator` (struct :`Pitch` -15.0) (`KismetMathLibrary.MakeRotator` 0.0 (`KismetMathLibrary.FClamp` _relativerotation_pitch -50.0 10.0) _relativerotation_yaw) (`self.bAutoRotateCamera`)) false false))

(fn `RandomizeIDLEEngineRPM`
  (bind (_torquecurve _rpmidle _rpmmax _inertia _backtorque) (break `/Game/Vehicles/MuscleCarV2/Setup/Structures/S_Engine` (`self.Engine`)))
  (set `self.Engine` (make `/Game/Vehicles/MuscleCarV2/Setup/Structures/S_Engine` _torquecurve (`KismetMathLibrary.RandomFloatInRange` 900.0 1000.0) _rpmmax _inertia _backtorque)))

(fn `SetSteeringInput`
  (params (AxisValue :type "Float (double-precision)"))
  (bind _steeringangle (`self.SteeringAngle`))
  (bind _steeringanglemax (`self.SteeringAngleMax`))
  (if (!= AxisValue 0.0)
    (set `self.SteeringAngle` (`KismetMathLibrary.FClamp` (+ (* AxisValue (* (`self.DeltaSeconds`) 125.0)) (`self.SteeringAngle`)) (* _steeringanglemax -1.0) _steeringanglemax))
    (else
      (set `self.SteeringAngle` (* (`self.SteeringAngle`) 0.7))))
  (`SceneComponent.K2_SetRelativeRotation` (`self.TopLink_FL`) (`KismetMathLibrary.MakeRotator` 0.0 0.0 _steeringangle) false false)
  (`SceneComponent.K2_SetRelativeRotation` (`self.TopLink_FR`) (`KismetMathLibrary.MakeRotator` 0.0 0.0 _steeringangle) false false))

(fn `UpdateSuspensionsLength`
  (for _index (range 4)
    ;[1 1 1] Set Suspensions Length to max if wheels are touching the ground
    (if (`|GetArrayItem` (`self.bWheelContact`) _index)
      (bind _output (`|GetArrayItem` (`self.TopLinkComponent`) _index))
      (bind (_namedebugonly _restlength _travel) (break `/Game/Vehicles/MuscleCarV2/Setup/Structures/S_Suspension` (`|GetArrayItem` (`self.Suspension`) _index)))
      ;[1 1 1] Adjust the suspensions length (with the body position)
      (`KismetArrayLibrary.Array_Set` (`self.Length`) _index (`KismetMathLibrary.FClamp` (`KismetMathLibrary.VSize` (- (`SceneComponent.K2_GetComponentLocation` _output) (+ (`.Location` (`GameplayStatics.BreakHitResult` (`|GetArrayItem` (`self.HitResult`) _index))) (* (`SceneComponent.GetUpVector` _output) (`.Radius_2_31E569DA423D4B98C93673A340DDDC2B` (break `/Game/Vehicles/MuscleCarV2/Setup/Structures/S_Wheel` (`|GetArrayItem` (`self.Wheel`) _index))))))) (- _restlength _travel) (+ _restlength _travel)))
      (else
        (bind (_namedebugonly_2 _restlength_2 _travel_2) (break `/Game/Vehicles/MuscleCarV2/Setup/Structures/S_Suspension` (`|GetArrayItem` (`self.Suspension`) _index)))
        (`KismetArrayLibrary.Array_Set` (`self.Length`) _index (+ _restlength_2 _travel_2))))))

(fn `UpdateWheelLocation`
  (for _index (range 4)
    (`SceneComponent.K2_SetRelativeLocation` (select `int` _index :`0` (`self.Wheel_FL`) :`1` (`self.Wheel_FR`) :`2` (`self.Wheel_RL`) :`3` (`self.Wheel_RR`)) (`KismetMathLibrary.MakeVector` 0.0 0.0 (* (`|GetArrayItem` (`self.Length`) _index) -1.0)) false false)))

(fn `UserConstructionScript`)

(fn `WheelRotation`
  (for _index (range 4)
    (bind _output_x (`KismetMathLibrary.BreakVector` (`|GetArrayItem` (`self.WheelLinearVelocityLocal`) _index)))
    (`SceneComponent.K2_AddLocalRotation` (select `int` _index :`0` (`self.Wheel_FL`) :`1` (`self.Wheel_FR`) :`2` (`self.Wheel_RL`) :`3` (`self.Wheel_RR`)) (`KismetMathLibrary.MakeRotator` 0.0 (* (`KismetMathLibrary.RadiansToDegrees` (* (/ _output_x (/ (`.Radius_2_31E569DA423D4B98C93673A340DDDC2B` (break `/Game/Vehicles/MuscleCarV2/Setup/Structures/S_Wheel` (`|GetArrayItem` (`self.Wheel`) _index))) 10.0)) (`self.DeltaSeconds`))) (select `int` _index :`0` 1.0 :`1` -1.0 :`2` 1.0 :`3` -1.0 :!type "Float (single-precision)"))) false false)))

(fn `WheelsRayCast`
  (for _index (range 4)
    (bind _output (`|GetArrayItem` (`self.TopLinkComponent`) _index))
    (bind _returnvalue (`SceneComponent.K2_GetComponentLocation` _output))
    ;[1 1 1] Cast the Suspensions Length
    (bind (_outhit _returnvalue_2) (`KismetSystemLibrary.LineTraceSingle` :`Start` _returnvalue :`End` (- _returnvalue (* (`SceneComponent.GetUpVector` _output) 100.0)) :`TraceChannel` "TraceTypeQuery1" :`DrawDebugType` "ForOneFrame" :`DrawTime` 1.0))
    ;[1 1 1] Define if the wheels are touching the ground
    (`KismetArrayLibrary.Array_Set` (`self.bWheelContact`) _index _returnvalue_2)
    (if _returnvalue_2
      (`KismetArrayLibrary.Array_Set` (`self.HitResult`) _index _outhit))))