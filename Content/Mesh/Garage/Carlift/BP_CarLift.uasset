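; BP_CarLift is a garage car lift actor that posts an event at its location when its lift state changes.
; On BeginPlay it caches the skeletal mesh's ABP_CarLift anim instance.
; Tick polls that instance's ShouldLift flag and feeds two DoOnce gates that reset each other, so each state posts once rather than every frame.
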(event `self.ReceiveBeginPlay`
  (bind _asabp_car_lift (cast `/Game/Mesh/Garage/Carlift/ABP_CarLift` (`SkeletalMeshComponent.GetAnimInstance` (`self.SkeletalMesh`))))
  (set `self.ABPREF Car Lift` _asabp_car_lift))

(event `self.ReceiveTick`
  (params (DeltaSeconds :type "Float (single-precision)"))
  (bind _returnvalue (`self.K2_GetActorLocation`))
  (if (`/Game/Mesh/Garage/Carlift/ABP_CarLift.bShouldLift` (`self.ABPREF Car Lift`))
    (`/Engine/EditorBlueprintResources/StandardMacros.DoOnce` false :!label _label
      (:`Completed`
        (`AkGameplayStatics.PostEventAtLocation` null _returnvalue)
        (goto _label_2 :!via `Reset`)))
    (else
      (`/Engine/EditorBlueprintResources/StandardMacros.DoOnce` false :!label _label_2
        (:`Completed`
          (`AkGameplayStatics.PostEventAtLocation` null _returnvalue)
          (goto _label :!via `Reset`))))))

(fn `UserConstructionScript`)