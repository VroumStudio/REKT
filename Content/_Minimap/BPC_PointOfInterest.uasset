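; Actor component that marks its owner as a point of interest on the minimap.
; On BeginPlay it caches the BP_REKTGameMode reference.
; On Tick, once the owner is valid, a DoOnce passes it a single time to AddPOI on the minimap widget, reached through the game mode's main widget reference.
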(event `self.ReceiveBeginPlay`
  (bind _asbp_rektgame_mode (cast `/Game/Blueprints/Base/BP_REKTGameMode` (`GameplayStatics.GetGameMode`)))
  (set `self.BPREF_Gamemode` _asbp_rektgame_mode))

(event `self.ReceiveTick`
  (params (DeltaSeconds :type "Float (single-precision)"))
  (`/Engine/EditorBlueprintResources/StandardMacros.IsValid` (`self.GetOwner`)
    (:`Is Valid`
      (`/Engine/EditorBlueprintResources/StandardMacros.DoOnce` false
        (:`Completed`
          (`/Game/_Minimap/W_Minimap.AddPOI` (`/Game/Widgets/InGame/W_Main.W_Minimap` (`/Game/Blueprints/Base/BP_REKTGameMode.WREF_Main` (`self.BPREF_Gamemode`))) (`self.GetOwner`)))))))