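; BP_EquipementPlacementZone is a trigger zone marking where the player's master vehicle can place equipment.
; When a "Vehicle"-tagged actor overlaps its box, it shows a particle effect, enables placement on the vehicle and passes it the arrow's world transform.
; Any end overlap reverses this, restores normal time dilation, removes the turret placement widget and posts a Wwise normal-state event.
; The construction script scales the mesh in X and Y.
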(event `self.ReceiveBeginPlay`
  (bind _asbp_master_vehicle (cast `/Game/Vehicles/MasterVehicle/BP_MasterVehicle` (`GameplayStatics.GetPlayerPawn` 0)))
  (set `self.BPREF_MasterVehicle` _asbp_master_vehicle))

(event `self.ReceiveTick`
  (params (DeltaSeconds :type "Float (single-precision)")))

(event `self.Box.OnComponentBeginOverlap`
  (params (OverlappedComponent :type "PrimitiveComponent Object Reference") (OtherActor :type "Actor Object Reference") (OtherComp :type "PrimitiveComponent Object Reference") (OtherBodyIndex :type Integer) (bFromSweep :type Boolean) (SweepResult :type "HitResult Structure (by ref)"))
  (bind _bpref_mastervehicle (`self.BPREF_MasterVehicle`))
  (if (`self.ActorHasTag` OtherActor "Vehicle")
    (`SceneComponent.SetVisibility` (`self.ParticleSystem`) true false)
    (set `/Game/Vehicles/MasterVehicle/BP_MasterVehicle.bCanPlaceEquipement` true _bpref_mastervehicle)
    (set `/Game/Vehicles/MasterVehicle/BP_MasterVehicle.PlacementTransform` (`SceneComponent.K2_GetComponentToWorld` (`self.Arrow`)) _bpref_mastervehicle)))

(event `self.Box.OnComponentEndOverlap`
  (params (OverlappedComponent :type "PrimitiveComponent Object Reference") (OtherActor :type "Actor Object Reference") (OtherComp :type "PrimitiveComponent Object Reference") (OtherBodyIndex :type Integer))
  (bind _bpref_mastervehicle (`self.BPREF_MasterVehicle`))
  (`SceneComponent.SetVisibility` (`self.ParticleSystem`) false false)
  (set `/Game/Vehicles/MasterVehicle/BP_MasterVehicle.bCanPlaceEquipement` false _bpref_mastervehicle)
  (`GameplayStatics.SetGlobalTimeDilation` 1.0)
  (`Widget.RemoveFromParent` (`/Game/Vehicles/MasterVehicle/BP_MasterVehicle.WREF_TurretsPlacement` _bpref_mastervehicle))
  (`AkGameplayStatics.PostEvent` "/Game/Audio/AKEvents/Set_State_ST_Normal.Set_State_ST_Normal" self))

(fn `UserConstructionScript`
  (`SceneComponent.SetRelativeScale3D` (`self.StaticMesh`) (`KismetMathLibrary.MakeVector` (`self.ScaleX`) (`self.ScaleY`) 1.0)))