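; BP_MineTrap is a proximity mine trap that explodes when an actor tagged "Enemy" enters its trigger sphere.
; The construction script calls its parent and sizes the sphere from the Radius variable.
; On overlap it applies radial damage over three times that radius, spawns an explosion particle effect and destroys itself.
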(event `self.Mine_Radius.OnComponentBeginOverlap`
  (params (OverlappedComponent :type "PrimitiveComponent Object Reference") (OtherActor :type "Actor Object Reference") (OtherComp :type "PrimitiveComponent Object Reference") (OtherBodyIndex :type Integer) (bFromSweep :type Boolean) (SweepResult :type "HitResult Structure (by ref)"))
  (bind _returnvalue (`self.K2_GetActorLocation`))
  (if (`self.ActorHasTag` OtherActor "Enemy")
    (`GameplayStatics.ApplyRadialDamage` :`BaseDamage` (`self.Damages`) :`Origin` _returnvalue :`DamageRadius` (* (`self.Radius`) 3.0) :`DamageCauser` self :`InstigatedByController` null)
    (`GameplayStatics.SpawnEmitterAtLocation` "/Game/FX/Mine_Explosion/PS_Mine_Explosion.PS_Mine_Explosion" _returnvalue)
    (`self.K2_DestroyActor`)))

(fn `UserConstructionScript`
  (`parent.UserConstructionScript`)
  (`SphereComponent.SetSphereRadius` (`self.Mine_Radius`) (`self.Radius`) true))