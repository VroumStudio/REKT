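; BP_CircularSawTrap is a trap with three circular saw meshes that spin and damage actors they hit.
; A timeline started on BeginPlay drives the relative pitch of all three saws from one rotation track.
; Each saw's component hit event applies the Damage variable to the other actor, with the trap as damage causer.
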(event `self.ReceiveBeginPlay`
  (bind (_direction _rotator) (`Timeline|Timeline_0`)
    (:`Update`
      (`SceneComponent.K2_SetRelativeRotation` (`self.Saw01_Mesh`) (`KismetMathLibrary.MakeRotator` 0.0 _rotator) false false)
      (`SceneComponent.K2_SetRelativeRotation` (`self.Saw02_Mesh`) (`KismetMathLibrary.MakeRotator` 0.0 _rotator) false false)
      (`SceneComponent.K2_SetRelativeRotation` (`self.Saw03_Mesh`) (`KismetMathLibrary.MakeRotator` 0.0 _rotator) false false))))

(event `self.Saw01_Mesh.OnComponentHit`
  (params (HitComponent :type "PrimitiveComponent Object Reference") (OtherActor :type "Actor Object Reference") (OtherComp :type "PrimitiveComponent Object Reference") (NormalImpulse :type "Vector Structure") (Hit :type "HitResult Structure (by ref)"))
  (`GameplayStatics.ApplyDamage` OtherActor (`self.Damage`) null self))

(event `self.Saw02_Mesh.OnComponentHit`
  (params (HitComponent :type "PrimitiveComponent Object Reference") (OtherActor :type "Actor Object Reference") (OtherComp :type "PrimitiveComponent Object Reference") (NormalImpulse :type "Vector Structure") (Hit :type "HitResult Structure (by ref)"))
  (`GameplayStatics.ApplyDamage` OtherActor (`self.Damage`) null self))

(event `self.Saw03_Mesh.OnComponentHit`
  (params (HitComponent :type "PrimitiveComponent Object Reference") (OtherActor :type "Actor Object Reference") (OtherComp :type "PrimitiveComponent Object Reference") (NormalImpulse :type "Vector Structure") (Hit :type "HitResult Structure (by ref)"))
  (`GameplayStatics.ApplyDamage` OtherActor (`self.Damage`) null self))

(fn `UserConstructionScript`
  (`parent.UserConstructionScript`))