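; Proximity mine trap equipment that damages an enemy entering its range, then destroys itself.
; Sphere overlaps track an actor tagged "Ennemy", and the construction script sizes that sphere from Range.
; Tick fires a DoOnce that triggers the mine's animation Blueprint, waits, damages the currently tracked actor, then destroys the mine.
; Target-component search helpers are defined but not called by the trigger logic.
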(event `ApplyDamage`
  (params (HitActor :type "Actor Object Reference"))
  (`/Game/Blueprints/Ennemies/BPL_EnnemyDamaging.DamageEnnemy` HitActor (`self.Damage`)))

(event `self.ReceiveTick`
  (params (DeltaSeconds :type "Float (single-precision)"))
  (if (`self.bCanReceiveDamage`)
    (`/Engine/EditorBlueprintResources/StandardMacros.DoOnce` false
      (:`Completed`
        (bind _asmine_trap_anim_bp (cast `/Game/Traps/Mine_trap/Mine_Trap_Anim_BP` (`SkeletalMeshComponent.GetAnimInstance` (`self.EquipmentMesh`))))
        (set `/Game/Traps/Mine_trap/Mine_Trap_Anim_BP.Is Triggered` true _asmine_trap_anim_bp)
        (`KismetSystemLibrary.Delay` 2.0)
        (`self.ApplyDamage` (`self.ActorToDamage`))
        (`KismetSystemLibrary.Delay` 1.0)
        (`self.K2_DestroyActor`)))))

(event `self.SphereRange.OnComponentBeginOverlap`
  (params (OverlappedComponent :type "PrimitiveComponent Object Reference") (OtherActor :type "Actor Object Reference") (OtherComp :type "PrimitiveComponent Object Reference") (OtherBodyIndex :type Integer) (bFromSweep :type Boolean) (SweepResult :type "HitResult Structure (by ref)"))
  (if (`self.ActorHasTag` OtherActor "Ennemy")
    (set `self.bCanReceiveDamage` true)
    (set `self.ActorToDamage` OtherActor)))

(event `self.SphereRange.OnComponentEndOverlap`
  (params (OverlappedComponent :type "PrimitiveComponent Object Reference") (OtherActor :type "Actor Object Reference") (OtherComp :type "PrimitiveComponent Object Reference") (OtherBodyIndex :type Integer))
  (set `self.bCanReceiveDamage` false)
  (set `self.ActorToDamage` null))

(fn `FindFirstTarget`
  (returns (NewTarget :type "Actor Object Reference"))
  (locals (Target :type "Actor Object Reference"))
  (for _array_element (`PrimitiveComponent.GetOverlappingActors` (`self.SphereRange`) "/Script/Engine.Actor")
    (bind _targetcomponent (`self.GetTargetComponent` _array_element))
    (if (`KismetSystemLibrary.IsValid` _targetcomponent)
      (if (`/Game/Blueprints/Equipements/Setup/BP_TargetComponent.bIsDead` _targetcomponent)
        (set `local.Target` _array_element))))
  (return (`local.Target`)))

(fn `GetTargetComponent`
  (params (CurrentTargetActor :type "Actor Object Reference"))
  (returns (TargetComponent :type "/Game/Blueprints/Equipements/Setup/BP_TargetComponent Object Reference"))
  (locals (Target :type "/Game/Blueprints/Equipements/Setup/BP_TargetComponent Object Reference"))
  (for _array_element (`self.K2_GetComponentsByClass` CurrentTargetActor "/Game/Blueprints/Equipements/Setup/BP_TargetComponent.BP_TargetComponent_C")
    (if (`KismetSystemLibrary.IsValid` _array_element)
      (set `local.Target` _array_element)))
  (return (`local.Target`)))

(fn `UserConstructionScript`
  (`SphereComponent.SetSphereRadius` (`self.SphereRange`) (* (`self.Range`) 2.0 100.0) true))