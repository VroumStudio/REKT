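; Gatling turret Blueprint that turns to face its target actor and fires at it.
; Each Tick caches the Scene component's world location and rotation as the fire transform, with unit scale.
; While it has a target, it aims poseable mesh bones in world space via look-at rotations, yaw only for the horizontal rotator and full rotation for the vertical one.
; It then calls Fire every frame; target selection is not handled in this graph.
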(event `self.ReceiveTick`
  (params (DeltaSeconds :type "Float (single-precision)"))
  (bind _poseablemesh (`self.PoseableMesh`))
  (bind _poseablemesh_2 (`self.PoseableMesh`))
  (bind _returnvalue (`self.K2_GetActorLocation` (`self.TargetActor`)))
  (bind (_returnvalue_location _returnvalue_rotation) (`KismetMathLibrary.BreakTransform` (`SceneComponent.K2_GetComponentToWorld` (`self.Scene`))))
  (set `self.FireTrasnform` (`KismetMathLibrary.MakeTransform` _returnvalue_location _returnvalue_rotation))
  (if (`self.bHasTarget`)
    (bind _returnvalue_2 (`PoseableMeshComponent.GetBoneLocationByName` _poseablemesh_2 "Horizontal_Rotator" "WorldSpace"))
    (bind (_returnvalue_roll _returnvalue_pitch _returnvalue_yaw) (`KismetMathLibrary.BreakRotator` (`KismetMathLibrary.FindLookAtRotation` _returnvalue_2 _returnvalue)))
    (`PoseableMeshComponent.SetBoneRotationByName` _poseablemesh_2 "Horizontal_Rotator" (`KismetMathLibrary.MakeRotator` 0.0 0.0 _returnvalue_yaw) "WorldSpace")
    (bind _returnvalue_3 (`PoseableMeshComponent.GetBoneLocationByName` _poseablemesh "Vertical_Rotator" "WorldSpace"))
    (bind (_returnvalue_roll_2 _returnvalue_pitch_2 _returnvalue_yaw_2) (`KismetMathLibrary.BreakRotator` (`KismetMathLibrary.FindLookAtRotation` _returnvalue_3 _returnvalue)))
    (`PoseableMeshComponent.SetBoneRotationByName` _poseablemesh "Vertical_Rotator" (`KismetMathLibrary.MakeRotator` _returnvalue_roll_2 _returnvalue_pitch_2 _returnvalue_yaw_2) "WorldSpace")
    (`self.Fire`)))

(fn `UserConstructionScript`
  (`parent.UserConstructionScript`))