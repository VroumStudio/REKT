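; Shotgun turret Blueprint that materializes on spawn and fires at its target actor.
; BeginPlay creates a dynamic material, and after a short delay a timeline drives its Dissolve parameter, then flags the turret as spawned.
; While the target is valid, Tick uses a DoOnce and FireRate delay to loop muzzle effects on three cannon sockets.
; A separate event, not called in this graph, applies damage to the target.
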(event `self.ReceiveBeginPlay`
  (`parent.ReceiveBeginPlay`)
  (bind _returnvalue (`PrimitiveComponent.CreateDynamicMaterialInstance` (`self.PoseableMesh`) 0 "/Game/Turrets/ShotGun_Turret/MI_ShotGun_Turret.MI_ShotGun_Turret" "None"))
  (set `self.DMI_ShotGun_Turret` _returnvalue)
  (`KismetSystemLibrary.Delay` 1.1)
  (bind (_direction _dissolve) (`Timeline|ShotGun_Turret_Apparition` :!via `PlayFromStart`)
    (:`Update`
      (`MaterialInstanceDynamic.SetScalarParameterValue` (`self.DMI_ShotGun_Turret`) "Dissolve" _dissolve))
    (:`Finished`
      (set `self.Is spawned` true))))

(event `EVNT_ApplyDamage_1`
  (`KismetSystemLibrary.Delay` 0.0)
  (`GameplayStatics.ApplyDamage` (`self.TargetActor`) (`self.Damage`) null self))

(event `self.ReceiveTick`
  (params (DeltaSeconds :type "Float (single-precision)"))
  (bind _poseablemesh (`self.PoseableMesh`))
  (`/Engine/EditorBlueprintResources/StandardMacros.IsValid` (`self.TargetActor`)
    (:`Is Valid`
      (set `self.Is firing` true)
      (`/Engine/EditorBlueprintResources/StandardMacros.DoOnce` false :!label _label
        (:`Completed`
          (`KismetSystemLibrary.Delay` (`self.FireRate`))
          (`GameplayStatics.SpawnEmitterAttached` "/Game/FX/FX_Shotgun/PS_ShotGun_Shot.PS_ShotGun_Shot" _poseablemesh "Socket_Cannon" (0.0 0.0 0.0) (struct :`Yaw` 90.0))
          (`GameplayStatics.SpawnEmitterAttached` "/Game/FX/FX_Shotgun/PS_ShotGun_Shot.PS_ShotGun_Shot" _poseablemesh "Socket_Cannon_0" (0.0 0.0 0.0) (struct :`Yaw` 90.0))
          (`GameplayStatics.SpawnEmitterAttached` "/Game/FX/FX_Shotgun/PS_ShotGun_Shot.PS_ShotGun_Shot" _poseablemesh "Socket_Cannon_1" (0.0 0.0 0.0) (struct :`Yaw` 90.0))
          (`KismetSystemLibrary.Delay` 0.2)
          (goto _label :!via `Reset`))))
    (:`Is Not Valid`
      (set `self.Is firing` false))))

(fn `UserConstructionScript`
  (`parent.UserConstructionScript`))