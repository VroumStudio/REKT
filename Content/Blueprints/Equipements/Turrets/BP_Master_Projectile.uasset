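; Master projectile Blueprint for turrets that deals area and direct damage on impact and has a two-second lifetime.
; BeginPlay sizes its collision sphere and caches the first BP_MasterTurret found in the level, not necessarily the one that fired it.
; Any hit applies radial damage; Enemy-tagged actors also take direct damage, trigger that turret's emitter event and destroy the projectile.
; A Delay on Tick handles the timed self-destruction.
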(event `self.ReceiveBeginPlay`
  (`SphereComponent.SetSphereRadius` (`self.Sphere`) (`self.Projectile_Radius`) true)
  (bind _outactors (`GameplayStatics.GetAllActorsOfClass` "/Game/Blueprints/Equipements/Turrets/BP_MasterTurret.BP_MasterTurret_C"))
  (set `self.BP_Master_Turret` (`|GetArrayItem` _outactors)))

(event `self.ReceiveActorBeginOverlap`
  (params (OtherActor :type "Actor Object Reference")))

(event `self.ReceiveTick`
  (params (DeltaSeconds :type "Float (single-precision)"))
  (`KismetSystemLibrary.Delay` 2.0)
  (`self.K2_DestroyActor`))

(event `self.Sphere.OnComponentHit`
  (params (HitComponent :type "PrimitiveComponent Object Reference") (OtherActor :type "Actor Object Reference") (OtherComp :type "PrimitiveComponent Object Reference") (NormalImpulse :type "Vector Structure") (Hit :type "HitResult Structure (by ref)"))
  (`GameplayStatics.ApplyRadialDamage` :`BaseDamage` (`self.Damage`) :`Origin` (`.Location` (`GameplayStatics.BreakHitResult` Hit)) :`DamageRadius` (`self.Aoe`) :`DamageCauser` null :`InstigatedByController` null :`bDoFullDamage` true)
  (if (`self.ActorHasTag` OtherActor "Enemy")
    (`GameplayStatics.ApplyDamage` OtherActor (`self.Damage`))
    (`/Game/Blueprints/Equipements/Turrets/BP_MasterTurret.EVNT_Emitter` (`self.BP_Master_Turret`))
    (`self.K2_DestroyActor`)))

(fn `UserConstructionScript`)