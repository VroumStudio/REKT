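; Base turret Blueprint that detects "Ennemy"-tagged actors within a range sphere sized from Range in the construction script.
; Overlap events set or clear the current target, with any actor's exit clearing it.
; Fire spawns a projectile and re-calls itself every FireRate delay, though nothing here starts it or reads the target.
; An uncalled FindFirstTarget helper returns an overlapping actor whose BP_TargetComponent is flagged IsDead.
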(event `self.ReceiveBeginPlay`
  (`KismetSystemLibrary.Delay` 0.8)
  (`SceneComponent.SetVisibility` (`self.PoseableMesh`) true true))

(event `self.SphereRange.OnComponentBeginOverlap`
  (params (OverlappedComponent :type "PrimitiveComponent Object Reference") (OtherActor :type "Actor Object Reference") (OtherComp :type "PrimitiveComponent Object Reference") (OtherBodyIndex :type Integer) (bFromSweep :type Boolean) (SweepResult :type "HitResult Structure (by ref)"))
  (if (`self.ActorHasTag` OtherActor "Ennemy")
    (set `self.bHasTarget` true)
    (set `self.TargetActor` OtherActor)))

(event `self.SphereRange.OnComponentEndOverlap`
  (params (OverlappedComponent :type "PrimitiveComponent Object Reference") (OtherActor :type "Actor Object Reference") (OtherComp :type "PrimitiveComponent Object Reference") (OtherBodyIndex :type Integer))
  (set `self.bHasTarget` false)
  (set `self.TargetActor` null))

(event `Fire`
  (bind (_firetrasnform_location _firetrasnform_rotation) (`KismetMathLibrary.BreakTransform` (`self.FireTrasnform`)))
  (`|SpawnActorFromClass` (`self.Projectile`) (`KismetMathLibrary.MakeTransform` _firetrasnform_location _firetrasnform_rotation) "Undefined" "OverrideRootScale" null null)
  (`KismetSystemLibrary.Delay` (`self.FireRate`))
  (`self.Fire`))

(fn `FindFirstTarget`
  (returns (NewTarget :type "Actor Object Reference"))
  (locals (Target :type "Actor Object Reference"))
  (for _array_element (`PrimitiveComponent.GetOverlappingActors` (`self.SphereRange`) "/Script/Engine.Actor")
    (bind _targetcomponent (`self.GetTargetComponent` _array_element))
    (if (`KismetSystemLibrary.IsValid` _targetcomponent)
      (if (`/Game/Blueprints/Equipements/Setup/BP_TargetComponent.bIsDead` _targetcomponent)
        (set `local.Target` _array_element))))
  (return (`local.Target`)))

(fn `GetTargetComponent`
  (params (CurrentTargetActor :type "Actor Object Reference"))
  (returns (TargetComponent :type "/Game/Blueprints/Equipements/Setup/BP_TargetComponent Object Reference"))
  (locals (Target :type "/Game/Blueprints/Equipements/Setup/BP_TargetComponent Object Reference"))
  (for _array_element (`self.K2_GetComponentsByClass` CurrentTargetActor "/Game/Blueprints/Equipements/Setup/BP_TargetComponent.BP_TargetComponent_C")
    (if (`KismetSystemLibrary.IsValid` _array_element)
      (set `local.Target` _array_element)))
  (return (`local.Target`)))

(fn `UserConstructionScript`
  (`SphereComponent.SetSphereRadius` (`self.SphereRange`) (* (`self.Range`) 2.0 100.0) true))