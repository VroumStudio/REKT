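; Laser turret that fades in on spawn through a timeline-driven Dissolve material parameter, then flags itself as spawned.
; While a target is valid, Tick uses a DoOnce reset after FireRate to play the charge effect and shot sound, clearing both effect and firing flag when the target is lost.
; A separate event applies delayed radial damage around the target; target acquisition is not handled here.
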(event `self.ReceiveBeginPlay`
  (`parent.ReceiveBeginPlay`)
  (bind _returnvalue (`PrimitiveComponent.CreateDynamicMaterialInstance` (`self.PoseableMesh`) 0 "/Game/Turrets/Laser_Turret/MI_Laser_Turret.MI_Laser_Turret" "None"))
  (set `self.DMI_LaserTurret` _returnvalue)
  (`KismetSystemLibrary.Delay` 1.1)
  (bind (_direction _dissolve) (`Timeline|Laser_Turret_Apparition` :!via `PlayFromStart`)
    (:`Update`
      (`MaterialInstanceDynamic.SetScalarParameterValue` (`self.DMI_LaserTurret`) "Dissolve" _dissolve))
    (:`Finished`
      (set `self.Is spawned` true))))

(event `self.ReceiveTick`
  (params (DeltaSeconds :type "Float (single-precision)"))
  (`/Engine/EditorBlueprintResources/StandardMacros.IsValid` (`self.TargetActor`)
    (:`Is Valid`
      (`/Engine/EditorBlueprintResources/StandardMacros.DoOnce` false :!label _label
        (:`Completed`
          (set `self.Is firing` true)
          (bind _returnvalue (`GameplayStatics.SpawnEmitterAttached` "/Game/FX/FX_Laser_Turret/PS_Laser_Charge.PS_Laser_Charge" (`self.PoseableMesh`) "Laser_Cannon" (0.0 0.0 0.0) (struct :`Yaw` 90.0)))
          (`AkGameplayStatics.PostEvent` "/Game/Audio/AKEvents/SFX/Turret/Play_SFX_Turret_Laser_Shoot.Play_SFX_Turret_Laser_Shoot" self)
          (`KismetSystemLibrary.PrintString` "FX" true true (struct :`G` 1.0 :`A` 1.0))
          (`KismetSystemLibrary.Delay` (`self.FireRate`))
          (goto _label :!via `Reset`))))
    (:`Is Not Valid`
      (set `self.Is firing` false)
      (`/Engine/EditorBlueprintResources/StandardMacros.IsValid` _returnvalue
        (:`Is Valid`
          (`ActorComponent.K2_DestroyComponent` _returnvalue))))))

(event `EVNT_ApplyDamage_1`
  (`KismetSystemLibrary.Delay` 0.5)
  (`GameplayStatics.ApplyRadialDamage` :`BaseDamage` (`self.Damage`) :`Origin` (+ (`self.K2_GetActorLocation` (`self.TargetActor`)) (0.0 0.0 50.0)) :`DamageRadius` (`self.Radius`) :`DamageTypeClass` "/Script/Engine.DamageType" :`DamageCauser` self :`InstigatedByController` null :`bDoFullDamage` true)
  (`KismetSystemLibrary.PrintString` "Apply damage" true true (struct :`R` 1.0 :`B` 1.0 :`A` 1.0)))

(fn `UserConstructionScript`
  (`parent.UserConstructionScript`))