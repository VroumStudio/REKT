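; Base turret projectile that damages actors tagged "Enemy" on impact.
; Its sphere's hit event calls OnDamagingActor with the hit actor and Damage for enemies, then destroys the projectile whatever it struck.
; Construction sizes the sphere from CollisionRadius, and a Delay driven from Tick destroys the projectile after a short lifetime.
; An area-of-effect radial damage node is present but never runs.
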(event `self.ReceiveTick`
  (params (DeltaSeconds :type "Float (single-precision)"))
  (`/Engine/EditorBlueprintResources/StandardMacros.IsValid` self
    (:`Is Valid`
      (`KismetSystemLibrary.Delay` 2.0)
      (`self.K2_DestroyActor`))))

(event `self.Sphere.OnComponentHit`
  (params (HitComponent :type "PrimitiveComponent Object Reference") (OtherActor :type "Actor Object Reference") (OtherComp :type "PrimitiveComponent Object Reference") (NormalImpulse :type "Vector Structure") (Hit :type "HitResult Structure (by ref)"))
  (if (`self.ActorHasTag` OtherActor "Enemy")
    (`/Game/Blueprints/Ennemies/BPL_HealthDamaging.OnDamagingActor` OtherActor (`self.Damage`))
    (`self.K2_DestroyActor`)
    (else
      (`self.K2_DestroyActor`))))

(fn `UserConstructionScript`
  (`SphereComponent.SetSphereRadius` (`self.Sphere`) (`self.CollisionRadius`) true))