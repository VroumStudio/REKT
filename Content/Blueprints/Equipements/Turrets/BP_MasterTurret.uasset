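; Base turret actor that plays a timed drop-in sequence with camera shake and sound, then tracks Enemy-tagged actors.
; A range sphere, sized from Range at construction, sets the target and opens or closes a gate on a looping fire timer.
; Firing spawns projectiles at listed bones, gated by IsSpawned and IsFiring, which are never set true here.
; A second timer aims two PoseableMesh rotator bones, leading the target horizontally.
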(event `self.ReceiveBeginPlay`
  ;[1 1 1] Emitter timing
  (set `self.Is spawned` false)
  (`KismetSystemLibrary.Delay` 0.6)
  (`GameplayStatics.PlayWorldCameraShake` "/Game/CameraShake_Vibration/Turret_Spawn_Camera_Shake.Turret_Spawn_Camera_Shake_C" (`SceneComponent.K2_GetComponentLocation` (`self.ParticleSystem`)) 0.0 2000.0)
  (`AkGameplayStatics.PostEvent` "/Game/Audio/AKEvents/SFX/Turret/Play_SFX_Turret_Drop.Play_SFX_Turret_Drop" self)
  (`KismetSystemLibrary.Delay` 0.5)
  (`SceneComponent.SetVisibility` (`self.PoseableMesh`) true false)
  (`KismetSystemLibrary.K2_SetTimer` null "EVNT_TurretRotation" 0.1 true)
  (`AkGameplayStatics.PostEvent` "/Game/Audio/AKEvents/SFX/Turret/Play_SFX_Turret_Confirm.Play_SFX_Turret_Confirm" self))

(event `EVNT_Fire`
  (bind _poseablemesh (`self.PoseableMesh`))
  ;[1 1 1] Firing when a target is in range, stop firing when out of range
  (if (`self.Is spawned`)
    (if (`self.Is firing`)
      (`/Engine/EditorBlueprintResources/StandardMacros.Gate` true :!label _label
        (:`Exit`
          (for _array_element (`self.BonesToSpawnProjectile`)
            (`|SpawnActorFromClass` (`self.Projectile_Actor`) (`KismetMathLibrary.MakeTransform` (`SceneComponent.GetSocketLocation` _poseablemesh _array_element) (`SceneComponent.GetSocketRotation` _poseablemesh _array_element)) "Undefined" "OverrideRootScale" null null)
            (`KismetSystemLibrary.PrintString` "Damage" true true (struct :`R` 1.0 :`A` 1.0))))))))

(event `self.SphereRange.OnComponentBeginOverlap`
  (params (OverlappedComponent :type "PrimitiveComponent Object Reference") (OtherActor :type "Actor Object Reference") (OtherComp :type "PrimitiveComponent Object Reference") (OtherBodyIndex :type Integer) (bFromSweep :type Boolean) (SweepResult :type "HitResult Structure (by ref)"))
  ;[1 1 1] Firing when a target is in range, stop firing when out of range
  (if (`self.Is firing`)
    _
    (elif (`self.ActorHasTag` OtherActor "Enemy")
      (set `self.TargetActor` OtherActor)
      (`KismetSystemLibrary.K2_SetTimer` null "EVNT_Fire" (`self.FireRate`) true)
      (goto _label :!via `Open`))))

(event `self.SphereRange.OnComponentEndOverlap`
  (params (OverlappedComponent :type "PrimitiveComponent Object Reference") (OtherActor :type "Actor Object Reference") (OtherComp :type "PrimitiveComponent Object Reference") (OtherBodyIndex :type Integer))
  ;[1 1 1] Firing when a target is in range, stop firing when out of range
  (if (== (`self.TargetActor`) OtherActor)
    (set `self.TargetActor` null)
    (goto _label :!via `Close`)))

(event `EVNT_TurretRotation`
  (bind _targetactor (`self.TargetActor`))
  (`/Engine/EditorBlueprintResources/StandardMacros.IsValid` (`self.TargetActor`)
    (:`Is Valid`
      ;[1 1 1] Turret Rotation
      (`|ExecutionSequence`
        (:`then_0`
          (bind _returnvalue (`PoseableMeshComponent.GetBoneLocationByName` (`self.PoseableMesh`) "Horizontal_Rotator" "WorldSpace"))
          (bind _returnvalue_2 (`KismetMathLibrary.FindLookAtRotation` _returnvalue (- (+ (`self.K2_GetActorLocation` _targetactor) (* (`KismetMathLibrary.Normal` (`self.GetActorForwardVector` _targetactor)) (`self.Rotation_Anticipation`))) (0.0 0.0 200.0))))
          (set `self.HorizontalRotation` _returnvalue_2)
          (`PoseableMeshComponent.SetBoneRotationByName` (`self.PoseableMesh`) "Horizontal_Rotator" _returnvalue_2 "WorldSpace"))
        (:`then_1`
          (bind _returnvalue_3 (`PoseableMeshComponent.GetBoneLocationByName` (`self.PoseableMesh`) "Vertical_Rotator" "WorldSpace"))
          (bind _returnvalue_4 (`KismetMathLibrary.FindLookAtRotation` _returnvalue_3 (`self.K2_GetActorLocation` (`self.TargetActor`))))
          (set `self.VerticalRotation` _returnvalue_4)
          (`PoseableMeshComponent.SetBoneRotationByName` (`self.PoseableMesh`) "Vertical_Rotator" _returnvalue_4 "WorldSpace"))))))

(fn `UserConstructionScript`
  (`SphereComponent.SetSphereRadius` (`self.SphereRange`) (* (`self.Range`) 2.0 100.0) true))