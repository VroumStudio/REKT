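; BP_WormholeMeshSpawner is a wormhole actor that reveals its center and displaces surrounding spawnable objects when something enters its trigger box.
; Each tick it writes its location to the MPC_WormHole_Collection material parameter collection.
; On BeginPlay it gathers all BP_WormHoleSpawnableActor instances and creates a dynamic center material with its opacity parameter at zero.
; Box overlap restarts a timeline that drives the center opacity and each gathered actor's displacement material parameter.
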(event `self.ReceiveTick`
  (params (DeltaSeconds :type "Float (single-precision)"))
  (`KismetMaterialLibrary.SetVectorParameterValue` "/Game/Materials/Worm_Hole/MPC_WormHole_Collection.MPC_WormHole_Collection" "Texloc" (`KismetMathLibrary.Conv_VectorToLinearColor` (`self.K2_GetActorLocation`))))

(event `self.Box.OnComponentBeginOverlap`
  (params (OverlappedComponent :type "PrimitiveComponent Object Reference") (OtherActor :type "Actor Object Reference") (OtherComp :type "PrimitiveComponent Object Reference") (OtherBodyIndex :type Integer) (bFromSweep :type Boolean) (SweepResult :type "HitResult Structure (by ref)"))
  (bind (_direction _wormhole_center_opacity _wormhole_objects_displacement) (`Timeline|TL_WormHole_Opacity` :!via `PlayFromStart`)
    (:`Update`
      (`MaterialInstanceDynamic.SetScalarParameterValue` (`self.Wormhole_Opacity`) "Seed_WormHole_Center" _wormhole_center_opacity)
      (for _array_element (`self.Meshes`)
        (`MaterialInstanceDynamic.SetScalarParameterValue` (`/Game/Blueprints/BP_WormHoleSpawnableActor.WormHoleMatInstance` _array_element) "Seed_WormHole_Objects" _wormhole_objects_displacement)))))

(event `self.ReceiveBeginPlay`
  (bind _outactors (`GameplayStatics.GetAllActorsOfClass` "/Game/Blueprints/BP_WormHoleSpawnableActor.BP_WormHoleSpawnableActor_C"))
  (set `self.Meshes` _outactors)
  (bind _returnvalue (`PrimitiveComponent.CreateDynamicMaterialInstance` (`self.Wormhole_Center`) 0 "/Game/Materials/Worm_Hole/M_Center_Wormhole.M_Center_Wormhole" "None"))
  (set `self.Wormhole_Opacity` _returnvalue)
  (`MaterialInstanceDynamic.SetScalarParameterValue` (`self.Wormhole_Opacity`) "Seed_WormHole_Center" 0.0))

(fn `UserConstructionScript`)