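; Base turret placement spot that opens a placement or correction widget when the cursor moves over its mesh.
; On hover it removes both widgets, then shows W_ObjectCorrection if a turret is spawned, otherwise W_ObjectPlacement, and passes itself to that widget.
; The placement branch also stores a spawn transform raised above the mesh.
; BeginPlay caches the aerial pawn and turns off the mesh's custom depth.
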(event `self.ReceiveBeginPlay`
  (bind _asbp_aerial_pawn (cast `/Game/Blueprints/GameBasis/BP_AerialPawn` (`GameplayStatics.GetPlayerPawn` 0)))
  (set `self.BPREF_AerialPawn` _asbp_aerial_pawn)
  (`PrimitiveComponent.SetRenderCustomDepth` (`self.StaticMeshComponent`) false))

(event `self.StaticMeshComponent.OnBeginCursorOver`
  (params (TouchedComponent :type "PrimitiveComponent Object Reference"))
  (bind _staticmeshcomponent (`self.StaticMeshComponent`))
  (`Widget.RemoveFromParent` (`self.WREF_ObjectPlacement`))
  (`Widget.RemoveFromParent` (`self.WREF_ObjectCorrection`))
  (if (`self.bSpawnedTurret`)
    (bind _returnvalue (`|CreateWidget` "/Game/Widgets/Placement/W_ObjectCorrection.W_ObjectCorrection_C"))
    (set `self.WREF_ObjectCorrection` _returnvalue)
    (`UserWidget.AddToViewport` (`self.WREF_ObjectCorrection`) 0)
    (set `/Game/Widgets/Placement/W_ObjectCorrection.BPREF_ObjectPlacementMaster` self (`self.WREF_ObjectCorrection`))
    (else
      (`self.AddWidgetToViewport`)
      (set `self.SpawnTransofrm` (`KismetMathLibrary.MakeTransform` (+ (`SceneComponent.K2_GetComponentLocation` _staticmeshcomponent) (0.0 0.0 100.0)) (`SceneComponent.K2_GetComponentRotation` _staticmeshcomponent))))))

(fn `AddWidgetToViewport`
  (bind _returnvalue (`|CreateWidget` "/Game/Widgets/Placement/W_ObjectPlacement.W_ObjectPlacement_C"))
  (set `self.WREF_ObjectPlacement` _returnvalue)
  (`UserWidget.AddToViewport` (`self.WREF_ObjectPlacement`) 0)
  (set `/Game/Widgets/Placement/W_ObjectPlacement.BPREF_ObjectPlacementMaster` self (`self.WREF_ObjectPlacement`))
  (set `/Game/Widgets/Placement/W_ObjectCorrection.WREF_ObjectPlacement` (`self.WREF_ObjectPlacement`) (`self.WREF_ObjectCorrection`))
  (return))

(fn `UserConstructionScript`)