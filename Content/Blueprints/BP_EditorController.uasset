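; BP_EditorController is a utility Blueprint of standalone events for clearing enemies and moving the car to preset spots on the level, apparently as an editor or testing aid.
; ClearEnemies destroys the actors tagged "Enemy".
; Each teleport event takes the first actor tagged "Car" and sends it to a hardcoded location and rotation: start, parking, first jump, second line or last line.
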(event `ClearEnemies`
  (bind _outactors (`GameplayStatics.GetAllActorsWithTag` "Enemy"))
  (`self.K2_DestroyActor` _outactors))

(event `TP_Car_LastLine`
  (bind _outactors (`GameplayStatics.GetAllActorsWithTag` "Car"))
  (`self.K2_TeleportTo` (`|GetArrayItem` _outactors) (74209.0 -33494.0 -3191.0) (struct :`Yaw` 180.0)))

(event `TP_Car_Start`
  (bind _outactors (`GameplayStatics.GetAllActorsWithTag` "Car"))
  (`self.K2_TeleportTo` (`|GetArrayItem` _outactors) (-48296.0 -22314.0 13892.0) (struct :`Pitch` -25.0)))

(event `Car_TP_Parking`
  (bind _outactors (`GameplayStatics.GetAllActorsWithTag` "Car"))
  (`self.K2_TeleportTo` :`self` (`|GetArrayItem` _outactors) :`DestLocation` (42738.0 9339.0 0.0)))

(event `Car_TP_FirstJump`
  (bind _outactors (`GameplayStatics.GetAllActorsWithTag` "Car"))
  (`self.K2_TeleportTo` (`|GetArrayItem` _outactors) (33892.0 -23491.0 0.0) (struct :`Yaw` -180.0)))

(event `Car_TP_SecondLine`
  (bind _outactors (`GameplayStatics.GetAllActorsWithTag` "Car"))
  (`self.K2_TeleportTo` (`|GetArrayItem` _outactors) (-1790.0 9427.0 0.0) (struct :`Yaw` 360.0)))

(fn `UserConstructionScript`)