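; Master enemy Blueprint that handles damage, death and player rewards, caching the player's BP_MasterVehicle and the game mode on BeginPlay.
; Damage is reduced by Armor, and a lethal hit triggers death and calls the vehicle's combo reset event.
; Death updates the vehicle's score, currency and kill counters, plays HUD animations, and destroys the enemy.
; Explosion debris inherits vehicle velocity, while money-drop effects attach above the vehicle, stacked higher by combo count.
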(event `self.ReceiveBeginPlay`
  (bind _asbp_master_vehicle (cast `/Game/Vehicles/MasterVehicle/BP_MasterVehicle` (`GameplayStatics.GetPlayerPawn` 0)))
  (set `self.BPREF_MasterVehicle` _asbp_master_vehicle)
  (bind _asbp_rektgame_mode (cast `/Game/Blueprints/Base/BP_REKTGameMode` (`GameplayStatics.GetGameMode`)))
  (set `self.BPREF_GameMode` _asbp_rektgame_mode))

(event `self.ReceiveAnyDamage`
  (params (Damage :type "Float (single-precision)") (DamageType :type "DamageType Object Reference") (InstigatedBy :type "Controller Object Reference") (DamageCauser :type "Actor Object Reference"))
  (bind _returnvalue (- (`self.Health`) (- Damage (`self.Armor`))))
  (if (<= _returnvalue 0.0)
    (`self.EVNT_Death`)
    (`/Game/Vehicles/MasterVehicle/BP_MasterVehicle.EVNT_ResetCombo` (`self.BPREF_MasterVehicle`))
    (else
      (set `self.Health` _returnvalue))))

(event `EVNT_Death`
  (bind _bpref_mastervehicle (`self.BPREF_MasterVehicle`))
  (bind _bpref_mastervehicle_2 (`self.BPREF_MasterVehicle`))
  (bind _bpref_mastervehicle_3 (`self.BPREF_MasterVehicle`))
  (bind _bpref_mastervehicle_4 (`self.BPREF_MasterVehicle`))
  (bind _bpref_mastervehicle_5 (`self.BPREF_MasterVehicle`))
  (bind _body (`/Game/Vehicles/MasterVehicle/BP_MasterVehicle.Body` _bpref_mastervehicle_3))
  (set `/Game/Vehicles/MasterVehicle/BP_MasterVehicle.Score` (+ (`/Game/Vehicles/MasterVehicle/BP_MasterVehicle.Score` _bpref_mastervehicle) (`self.ScoreGiven`)) _bpref_mastervehicle)
  (`self.PlayScoreAnimation`)
  (set `/Game/Vehicles/MasterVehicle/BP_MasterVehicle.Currency` (+ (`/Game/Vehicles/MasterVehicle/BP_MasterVehicle.Currency` _bpref_mastervehicle) (`self.CurrencyGiven`)) _bpref_mastervehicle)
  (`self.PlayMoneyAnimation`)
  (set `/Game/Vehicles/MasterVehicle/BP_MasterVehicle.RemainingEnemies` (- (`/Game/Vehicles/MasterVehicle/BP_MasterVehicle.RemainingEnemies` _bpref_mastervehicle) 1) _bpref_mastervehicle)
  (`self.K2_DestroyActor`)
  (bind _returnvalue (`GameplayStatics.SpawnEmitterAtLocation` "/Game/FX/Minion_Explosion/PS_Minion_Explosion.PS_Minion_Explosion" (- (`self.K2_GetActorLocation`) (0.0 0.0 70.0))))
  (`ParticleSystemComponent.SetVectorParameter` _returnvalue "Debris_Speed" (* (`KismetMathLibrary.Normal` (`SceneComponent.GetForwardVector` (`/Game/Vehicles/MasterVehicle/BP_MasterVehicle.Body` _bpref_mastervehicle_5))) (`/Game/Vehicles/MasterVehicle/BP_MasterVehicle.Speed` _bpref_mastervehicle_5)))
  ;[1 1 1] Money_Drop
  (if (>= (`/Game/Vehicles/MasterVehicle/BP_MasterVehicle.ComboCounter` _bpref_mastervehicle_3) 20)
    (set `/Game/Vehicles/MasterVehicle/BP_MasterVehicle.ComboCounter` 0 _bpref_mastervehicle_3))
  (`GameplayStatics.SpawnEmitterAttached` "/Game/FX/FX_Money_Drop/PS_Money_Drop_V2.PS_Money_Drop_V2" _body "None" (+ (`SceneComponent.K2_GetComponentLocation` _body) (0.0 0.0 175.0) (`KismetMathLibrary.MakeVector` 0.0 0.0 (* (`/Game/Vehicles/MasterVehicle/BP_MasterVehicle.ComboCounter` _bpref_mastervehicle_3) 90.0))) (struct) (1.0 1.0 1.0) "KeepWorldPosition")
  (set `/Game/Vehicles/MasterVehicle/BP_MasterVehicle.ComboCounter` (+ (`/Game/Vehicles/MasterVehicle/BP_MasterVehicle.ComboCounter` _bpref_mastervehicle_2) 1) _bpref_mastervehicle_2)
  (set `/Game/Vehicles/MasterVehicle/BP_MasterVehicle.EnemiesKilled` (+ (`/Game/Vehicles/MasterVehicle/BP_MasterVehicle.EnemiesKilled` _bpref_mastervehicle_4) 1) _bpref_mastervehicle_4))

(event `Test1`)

(fn `PlayMoneyAnimation`
  (bind _wref_main (`/Game/Blueprints/Base/BP_REKTGameMode.WREF_Main` (`self.BPREF_GameMode`)))
  (`UserWidget.PlayAnimation` _wref_main (`/Game/Widgets/InGame/W_Main.TriggerMoney` _wref_main) 0.0 1 "Forward" 1.0))

(fn `PlayScoreAnimation`
  (bind _wref_main (`/Game/Blueprints/Base/BP_REKTGameMode.WREF_Main` (`self.BPREF_GameMode`)))
  (`UserWidget.PlayAnimation` _wref_main (`/Game/Widgets/InGame/W_Main.TriggerScore` _wref_main) 0.0 1 "Forward" 1.0))

(fn `UserConstructionScript`)