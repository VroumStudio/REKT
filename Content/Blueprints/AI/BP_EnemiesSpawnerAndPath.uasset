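; Trigger-box spawner that launches enemy waves during a vehicle race.
; An overlap by a Vehicle-tagged actor that passes CheckDirection briefly shows the next wave number, until waves match the tracker's lap count.
; Red, green and blue enemy totals are halved between random points in left and right area boxes.
; A delayed DoN loop macro staggers the AI spawns and increments the player vehicle's remaining-enemy count.
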(event `self.ReceiveBeginPlay`
  ;[1 1 1] Make references to necessary BPs
  (bind _outactors (`GameplayStatics.GetAllActorsOfClass` "/Game/Blueprints/Checkpoints/BP_Tracker.BP_Tracker_C"))
  (set `self.BPREF_Tracker` (`|GetArrayItem` _outactors))
  (bind _asbp_master_vehicle (cast `/Game/Vehicles/MasterVehicle/BP_MasterVehicle` (`GameplayStatics.GetPlayerPawn` 0)))
  (set `self.BPREF_MasterVehicle` _asbp_master_vehicle)
  (bind _asbp_rektgame_mode (cast `/Game/Blueprints/Base/BP_REKTGameMode` (`GameplayStatics.GetGameMode`)))
  (set `self.BPREF_Gamemode` _asbp_rektgame_mode))

(event `self.TriggerBox.OnComponentBeginOverlap`
  (params (OverlappedComponent :type "PrimitiveComponent Object Reference") (OtherActor :type "Actor Object Reference") (OtherComp :type "PrimitiveComponent Object Reference") (OtherBodyIndex :type Integer) (bFromSweep :type Boolean) (SweepResult :type "HitResult Structure (by ref)"))
  (bind _w_wavedisplayer (`/Game/Widgets/InGame/W_Main.W_WaveDisplayer` (`/Game/Blueprints/Base/BP_REKTGameMode.WREF_Main` (`self.BPREF_Gamemode`))))
  ;[1 1 1] Check for direction of the vehicle
  (if (and (`self.CheckDirection`) (`self.ActorHasTag` OtherActor "Vehicle"))
    ;[1 1 1] Only spawn a wave while in race (prevent last time spawning when finishing the race)
    (if (not (== (`self.CurrentWave`) (`/Game/Blueprints/Checkpoints/BP_Tracker.Laps` (`self.BPREF_Tracker`))))
      (`|ExecutionSequence`
        (:`then_0`
          (set `self.CurrentWave` (+ (`self.CurrentWave`) 1))
          (`Widget.SetVisibility` _w_wavedisplayer "Visible")
          (`TextBlock.SetText` (`/Game/Widgets/InGame/W_WaveDisplayer.TextBlock_Waves` _w_wavedisplayer) (`|FormatText` "Wave {Wave}" (`self.CurrentWave`)))
          (`UserWidget.PlayAnimation` _w_wavedisplayer (`/Game/Widgets/InGame/W_WaveDisplayer.Appearance` _w_wavedisplayer) 0.0 1 "Forward" 1.0)
          (`KismetSystemLibrary.Delay` 2.0)
          (`Widget.SetVisibility` _w_wavedisplayer "Hidden"))
        (:`then_1`
          (`self.SpawnEnemies` (`self.SpawnPerLaps` (`self.RedEnemiesAmount`)) (`self.RedEnemiesClass`) (`self.RandomSpawnPointLeft`) 0.1))
        (:`then_2`
          (`self.SpawnEnemies` (`self.SpawnPerLaps` (`self.GreenEnemiesAmount`)) (`self.GreenEnemiesClass`) (`self.RandomSpawnPointLeft`) 0.1))
        (:`then_3`
          (`self.SpawnEnemies` (`self.SpawnPerLaps` (`self.BlueEnemiesAmount`)) (`self.BlueEnemiesClass`) (`self.RandomSpawnPointLeft`) 0.1))
        (:`then_4`
          (`self.SpawnEnemies` (`self.SpawnPerLaps` (`self.RedEnemiesAmount`)) (`self.RedEnemiesClass`) (`self.RandomSpawnPointRight`) 0.1))
        (:`then_5`
          (`self.SpawnEnemies` (`self.SpawnPerLaps` (`self.GreenEnemiesAmount`)) (`self.GreenEnemiesClass`) (`self.RandomSpawnPointRight`) 0.1))
        (:`then_6`
          (`self.SpawnEnemies` (`self.SpawnPerLaps` (`self.BlueEnemiesAmount`)) (`self.BlueEnemiesClass`) (`self.RandomSpawnPointRight`) 0.1))))))

(fn `RandomSpawnPointLeft`
  (returns (RandomLocation :type "Vector Structure"))
  (bind _areaboxleft (`self.AreaBoxLeft`))
  (return (`KismetMathLibrary.RandomPointInBoundingBox` (`SceneComponent.K2_GetComponentLocation` _areaboxleft) (`BoxComponent.BoxExtent` _areaboxleft))))

(fn `RandomSpawnPointRight`
  (returns (RandomLocation :type "Vector Structure"))
  (bind _areaboxright (`self.AreaBoxRight`))
  (return (`KismetMathLibrary.RandomPointInBoundingBox` (`SceneComponent.K2_GetComponentLocation` _areaboxright) (`BoxComponent.BoxExtent` _areaboxright))))

(fn `SpawnPerLaps`
  (params (EnemiesAmount :type Integer))
  (returns (FinalEnemiesToSpawn :type Integer))
  (return (/ EnemiesAmount 2)))

(fn `UserConstructionScript`)