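; BP_MenuPawn is a pawn that handles menu input for navigating to and within race selection.
; Start finds the aerial camera named RaceSelection, blends the player's view to it, clears all widgets and shows a new level selection widget.
; Validate and Cancel input are forwarded to that widget's custom start and cancel functions.
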(event `InputAction|Start`
  (params (Key :type "Key Structure"))
  (:`Pressed`
    (bind _outactors (`GameplayStatics.GetAllActorsOfClass` "/Game/Blueprints/Base/BP_AerialCamera.BP_AerialCamera_C"))
    (for _array_element _outactors
      (if (== (`/Game/Blueprints/Base/BP_AerialCamera.CameraName` _array_element) "RaceSelection")
        (`PlayerController.SetViewTargetWithBlend` (`GameplayStatics.GetPlayerController` 0) _array_element 1.0 "VTBlend_Cubic" 0.0 false)
        (`WidgetLayoutLibrary.RemoveAllWidgets`)
        (bind _returnvalue (`|CreateWidget` "/Game/Widgets/MainMenu/RaceSelection/W_LevelSelection.W_LevelSelection_C"))
        (bind _output_get (set `self.WREF_LevelSelection` _returnvalue))
        (`UserWidget.AddToViewport` _output_get 0)))))

(event `InputAction|Validate`
  (params (Key :type "Key Structure"))
  (:`Pressed`
    (`/Game/Widgets/MainMenu/RaceSelection/W_LevelSelection.CustomStart` (`self.WREF_LevelSelection`))))

(event `InputAction|Cancel`
  (params (Key :type "Key Structure"))
  (:`Pressed`
    (`/Game/Widgets/MainMenu/RaceSelection/W_LevelSelection.CustomCancel` (`self.WREF_LevelSelection`))))

(fn `UserConstructionScript`)