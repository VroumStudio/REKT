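; Base placeable turret unit that locks onto actors tagged "Ennemy" or "Targetable" when they overlap its Range.
; The construction script applies the configured skeletal mesh and animation Blueprint to the Turret.
; A Firing event, not called here, spawns the projectile class at the Canon_Socket after a short delay.
; It caches the player's aerial pawn, but the placement-point cost check and fire-rate logic are unwired.
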(event `self.ReceiveBeginPlay`
  (bind _asbp_aerial_pawn (cast `/Game/Blueprints/GameBasis/BP_AerialPawn` (`GameplayStatics.GetPlayerPawn` 0)))
  (set `self.BPREF_Pawn` _asbp_aerial_pawn)
  (set `self.Cost` (`self.Cost`)))

(event `self.Range.OnComponentBeginOverlap`
  (params (OverlappedComponent :type "PrimitiveComponent Object Reference") (OtherActor :type "Actor Object Reference") (OtherComp :type "PrimitiveComponent Object Reference") (OtherBodyIndex :type Integer) (bFromSweep :type Boolean) (SweepResult :type "HitResult Structure (by ref)"))
  (if (or (`self.ActorHasTag` OtherActor "Ennemy") (`self.ActorHasTag` OtherActor "Targetable"))
    (set `self.Target` OtherActor)
    (set `self.bLockedTarget` true)))

(event `self.Range.OnComponentEndOverlap`
  (params (OverlappedComponent :type "PrimitiveComponent Object Reference") (OtherActor :type "Actor Object Reference") (OtherComp :type "PrimitiveComponent Object Reference") (OtherBodyIndex :type Integer))
  (set `self.bLockedTarget` false))

(event `self.ReceiveTick`
  (params (DeltaSeconds :type "Float (single-precision)")))

(event `Firing`
  (`KismetSystemLibrary.Delay` 0.2)
  (`|SpawnActorFromClass` (`self.ProjectileClass`) (`SceneComponent.GetSocketTransform` (`self.Mesh`) "Canon_Socket" "RTS_World") "Undefined" "OverrideRootScale" null null))

(fn `UserConstructionScript`
  (bind _turret (`self.Turret`))
  (`SkinnedMeshComponent.SetSkinnedAssetAndUpdate` _turret (`self.TurretMesh`) true)
  (`SkeletalMeshComponent.K2_SetAnimInstanceClass` _turret (`self.AnimationBlueprint`))
  (set `self.ProjectileClass` (`self.ProjectileClass`)))