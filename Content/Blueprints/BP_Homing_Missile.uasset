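; BP_Homing_Missile is a projectile actor that can seek a target and explodes on contact.
; The Homing_Missile event takes a target and, if valid, sets its static mesh component as the homing target and enables strong homing acceleration on the projectile movement.
; The first sphere hit fires a radial force impulse, spawns an explosion particle effect and destroys the missile, guarded by a DoOnce.
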(event `self.Sphere.OnComponentHit`
  (params (HitComponent :type "PrimitiveComponent Object Reference") (OtherActor :type "Actor Object Reference") (OtherComp :type "PrimitiveComponent Object Reference") (NormalImpulse :type "Vector Structure") (Hit :type "HitResult Structure (by ref)"))
  (bind _explosion_force (`self.Explosion_Force`))
  ;[1 1 1] Explode_On_Contact
  (`/Engine/EditorBlueprintResources/StandardMacros.DoOnce` false
    (:`Completed`
      (`RadialForceComponent.FireImpulse` _explosion_force)
      (`GameplayStatics.SpawnEmitterAtLocation` "/Game/Turrets/Gatling_Gun_Turrets/FX/PS_Explosion_HIT_Gatling.PS_Explosion_HIT_Gatling" (`SceneComponent.K2_GetComponentLocation` _explosion_force))
      (`self.K2_DestroyActor`))))

(event `Homing_Missile`
  (params (Target_To_Hit :type "StaticMeshActor Object Reference"))
  (bind _projectilemovement (`self.ProjectileMovement`))
  ;[1 1 1] Set homing Missile
  (if (`KismetSystemLibrary.IsValid` Target_To_Hit)
    (set `ProjectileMovementComponent.HomingTargetComponent` (`StaticMeshActor.StaticMeshComponent` Target_To_Hit) _projectilemovement)
    (set `ProjectileMovementComponent.bIsHomingProjectile` true _projectilemovement)
    (set `ProjectileMovementComponent.HomingAccelerationMagnitude` 10000.0 _projectilemovement)))

(fn `UserConstructionScript`)