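; Master enemy Blueprint that sets its skeletal mesh and animation class from variables in the construction script.
; Each Tick it polls the health management component's IsDead flag, spawning a splat effect and destroying the actor on death, and prints Health as debug output.
; Overlap of its box by an actor tagged Vehicle kills it immediately with a blood sound and splat effect, bypassing the health check.
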(event `self.ReceiveTick`
  (params (DeltaSeconds :type "Float (single-precision)"))
  (bind (_returnvalue_location _returnvalue_rotation) (`KismetMathLibrary.BreakTransform` (`SceneComponent.K2_GetComponentToWorld` (`self.SkeletalMesh`))))
  (`|ExecutionSequence`
    (:`then_0`
      (if (`/Game/Blueprints/Ennemies/BPC_EnnemyHealthManagement.bIsDead` (`self.BPC_EnnemyHealthManagement`))
        (`/Engine/EditorBlueprintResources/StandardMacros.DoOnce` false
          (:`Completed`
            (`GameplayStatics.SpawnEmitterAtLocation` "/Game/FX/FX_Splat/Ps_Splat2.Ps_Splat2" _returnvalue_location _returnvalue_rotation)
            (`self.K2_DestroyActor`)))))
    (:`then_1`
      (`KismetSystemLibrary.PrintString` (`KismetStringLibrary.Concat_StrStr` "Health: " (`KismetStringLibrary.Conv_IntToString` (`self.Health`))) true true (struct :`G` 0.66 :`B` 1.0 :`A` 1.0) 0.0))))

(event `self.Box.OnComponentBeginOverlap`
  (params (OverlappedComponent :type "PrimitiveComponent Object Reference") (OtherActor :type "Actor Object Reference") (OtherComp :type "PrimitiveComponent Object Reference") (OtherBodyIndex :type Integer) (bFromSweep :type Boolean) (SweepResult :type "HitResult Structure (by ref)"))
  (bind (_returnvalue_location _returnvalue_rotation) (`KismetMathLibrary.BreakTransform` (`SceneComponent.K2_GetComponentToWorld` (`self.SkeletalMesh`))))
  (if (`self.ActorHasTag` OtherActor "Vehicle")
    (`/Engine/EditorBlueprintResources/StandardMacros.DoOnce` false
      (:`Completed`
        (`GameplayStatics.SpawnSoundAtLocation` "/Game/Audio/UE/SoundCues/Monster_Blood.Monster_Blood" _returnvalue_location (struct) 1.0 1.0 0.0 null null)
        (`GameplayStatics.SpawnEmitterAtLocation` "/Game/FX/FX_Splat/Ps_Splat2.Ps_Splat2" _returnvalue_location _returnvalue_rotation)
        (`self.K2_DestroyActor`)))))

(fn `UserConstructionScript`
  (bind _skeletalmesh (`self.SkeletalMesh`))
  (`SkinnedMeshComponent.SetSkinnedAssetAndUpdate` _skeletalmesh (`self.Mesh`) true)
  (`SkeletalMeshComponent.K2_SetAnimInstanceClass` _skeletalmesh (`self.Animation`)))