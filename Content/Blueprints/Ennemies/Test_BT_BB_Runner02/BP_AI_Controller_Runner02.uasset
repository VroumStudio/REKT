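; AI controller for the Runner02 enemy that moves its character along waypoint actors stored on the character.
; Every Tick it casts the controlled pawn, copies its Waypoint array and issues an AI MoveTo toward the current waypoint.
; On success, Patrolling increments the index and starts another move with no pawn wired in.
; Patrolling repeats only once the index reaches the last waypoint or beyond, and the index never resets.
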(event `self.ReceiveTick`
  (params (DeltaSeconds :type "Float (single-precision)"))
  (bind _asbp_ai_character_runner_02 (cast `/Game/Blueprints/Ennemies/Test_BT_BB_Runner02/BP_AI_Character_Runner02` (`self.K2_GetPawn`)))
  (set `self.Waypoints` (`/Game/Blueprints/Ennemies/Test_BT_BB_Runner02/BP_AI_Character_Runner02.Waypoint` _asbp_ai_character_runner_02))
  (`|AIMoveTo` _asbp_ai_character_runner_02 (0.0 0.0 0.0) (`|GetArrayItem` (`self.Waypoints`) (`self.CurrentWaypoint`))
    (:`OnSuccess`
      (`self.Patrolling`))))

(event `Patrolling`
  (`/Engine/EditorBlueprintResources/StandardMacros.IncrementInt` (`self.CurrentWaypoint`)
    (:`  `
      (`|AIMoveTo` null (0.0 0.0 0.0) (`|GetArrayItem` (`self.Waypoints`) (`self.CurrentWaypoint`))
        (:`OnSuccess`
          (if (>= (`self.CurrentWaypoint`) (- (`KismetArrayLibrary.Array_Length` (`self.Waypoints`)) 1))
            (`self.Patrolling`)))))))

(fn `UserConstructionScript`)