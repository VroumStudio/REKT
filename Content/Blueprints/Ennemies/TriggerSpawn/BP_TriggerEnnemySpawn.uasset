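; BP_TriggerEnnemySpawn is a trigger box actor that spawns an enemy when something overlaps it.
; The construction script sets the box's world scale from Scale and copies EnnemyClass into the class to spawn.
; Any overlap, with no filter or one-shot guard, starts a one-second delay, then spawns that class at the root component's transform and stores it in SpawnedEnnemy.
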(event `self.Box.OnComponentBeginOverlap`
  (params (OverlappedComponent :type "PrimitiveComponent Object Reference") (OtherActor :type "Actor Object Reference") (OtherComp :type "PrimitiveComponent Object Reference") (OtherBodyIndex :type Integer) (bFromSweep :type Boolean) (SweepResult :type "HitResult Structure (by ref)"))
  (`KismetSystemLibrary.Delay` 1.0)
  (bind _returnvalue (`|SpawnActorFromClass` (`self.Ennemy`) (`SceneComponent.K2_GetComponentToWorld` (`self.DefaultSceneRoot`)) "Undefined" "OverrideRootScale" null null))
  (set `self.SpawnedEnnemy` _returnvalue))

(fn `UserConstructionScript`
  (`SceneComponent.SetWorldScale3D` (`self.Box`) (`self.Scale`))
  (set `self.Ennemy` (`self.EnnemyClass`)))