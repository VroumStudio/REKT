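; Enemy actor from the wave-on-track set that travels along the spline of a referenced track.
; The EnnemyMove event scales a timeline's play rate by Duration and starts it from a per-enemy time offset.
; Each update maps the timeline alpha to a distance along the spline and sets the actor's world location and rotation from that point.
; BeginPlay, overlap and Tick hold no active logic.
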(event `EnnemyMove`
  (bind _returnvalue (`KismetMathLibrary.Lerp` 0.0 (`SplineComponent.GetSplineLength` (`/Game/Blueprints/Ennemies/SpawnWaveOnTrack/BP_Track.UsefullSpline` (`self.TrackReference`))) (`self.Alpha`)))
  (`TimelineComponent.SetPlayRate` (`self.EnnemyMoveTimeline`) (/ 1.0 (`self.Duration`)))
  (`TimelineComponent.SetNewTime` (`self.EnnemyMoveTimeline`) (`self.EnnemyStartOffset`))
  (bind (_direction _alpha) (`Timeline|EnnemyMoveTimeline`)
    (:`Update`
      (set `self.Alpha` _alpha)
      (`self.K2_SetActorLocationAndRotation` (`SplineComponent.GetLocationAtDistanceAlongSpline` (`/Game/Blueprints/Ennemies/SpawnWaveOnTrack/BP_Track.UsefullSpline` (`self.TrackReference`)) _returnvalue "World") (`SplineComponent.GetRotationAtDistanceAlongSpline` (`/Game/Blueprints/Ennemies/SpawnWaveOnTrack/BP_Track.UsefullSpline` (`self.TrackReference`)) _returnvalue "World")))))

(fn `UserConstructionScript`
  (`parent.UserConstructionScript`))