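; BP_TriggerEnemySpawn_OnTrack is a one-shot trigger box that spawns an enemy wave on tracks.
; On overlap, a DoOnce runs before the "Vehicle" tag check, so any first overlapping actor consumes the trigger.
; A vehicle overlap spawns three track enemy classes at world origin and calls EnnemyMove on each.
; The construction script caches the first "Track_1" actor as TrackReference, which the event graph never uses.
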(event `self.Box.OnComponentBeginOverlap`
  (params (OverlappedComponent :type "PrimitiveComponent Object Reference") (OtherActor :type "Actor Object Reference") (OtherComp :type "PrimitiveComponent Object Reference") (OtherBodyIndex :type Integer) (bFromSweep :type Boolean) (SweepResult :type "HitResult Structure (by ref)"))
  (`/Engine/EditorBlueprintResources/StandardMacros.DoOnce` false
    (:`Completed`
      (if (`self.ActorHasTag` OtherActor "Vehicle")
        (`|ExecutionSequence`
          (:`then_0`
            (bind _returnvalue (`|SpawnActorFromClass` "/Game/Blueprints/Ennemies/SpawnWaveOnTrack/BP_Ennemy_Track_1.BP_Ennemy_Track_1_C" (`KismetMathLibrary.MakeTransform` (0.0 0.0 0.0) (struct) (1.0 1.0 1.0)) "Undefined" "OverrideRootScale" null null))
            (`/Game/Blueprints/Ennemies/SpawnWaveOnTrack/BP_Ennemy_Track_1.EnnemyMove` _returnvalue))
          (:`then_1`
            (bind _returnvalue_2 (`|SpawnActorFromClass` "/Game/Blueprints/Ennemies/SpawnWaveOnTrack/BP_Ennemy_Track_2.BP_Ennemy_Track_2_C" (`KismetMathLibrary.MakeTransform` (0.0 0.0 0.0)) "Undefined" "OverrideRootScale" null null))
            (`/Game/Blueprints/Ennemies/SpawnWaveOnTrack/BP_Ennemy_Track_2.EnnemyMove` _returnvalue_2))
          (:`then_2`
            (bind _returnvalue_3 (`|SpawnActorFromClass` "/Game/Blueprints/Ennemies/SpawnWaveOnTrack/BP_Ennemy_Track_3.BP_Ennemy_Track_3_C" (`KismetMathLibrary.MakeTransform` (0.0 0.0 0.0)) "Undefined" "OverrideRootScale" null null))
            (`/Game/Blueprints/Ennemies/SpawnWaveOnTrack/BP_Ennemy_Track_3.EnnemyMove` _returnvalue_3)))))))

(fn `UserConstructionScript`
  (bind _outactors (`GameplayStatics.GetAllActorsWithTag` "Track_1"))
  (bind _asbp_track (cast `/Game/Blueprints/Ennemies/SpawnWaveOnTrack/BP_Track` (`|GetArrayItem` _outactors)))
  (set `self.TrackReference` _asbp_track))