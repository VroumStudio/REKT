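; Base enemy for wave spawning that loops through waypoints with AI MoveTo and can be run over by the player's vehicle.
; Overlapping a Vehicle-tagged actor scales down the player vehicle's velocity and triggers death, which adds score and currency, refills boost and destroys the enemy.
; Tick prints health and destroys the enemy at zero without those rewards.
; All three move events continue through EnemyMoveTo1; score multiplier logic is disconnected.
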(event `EnemyMoveTo1`
  (`|AIMoveTo` self (0.0 0.0 0.0) (`|GetArrayItem` (`self.Waypoints`) (`self.CurrentWaypoints`))
    (:`OnSuccess`
      (if (>= (`self.CurrentWaypoints`) (- (`KismetArrayLibrary.Array_Length` (`self.Waypoints`)) 1))
        (set `self.CurrentWaypoints` 0)
        (`self.EnemyMoveTo1`)
        (else
          (`/Engine/EditorBlueprintResources/StandardMacros.IncrementInt` (`self.CurrentWaypoints`)
            (:`  `
              (`self.EnemyMoveTo1`))))))))

(event `EnemyMoveTo2`
  (`|AIMoveTo` self (0.0 0.0 0.0) (`|GetArrayItem` (`self.Waypoints`) (`self.CurrentWaypoints`))
    (:`OnSuccess`
      (if (>= (`self.CurrentWaypoints`) (- (`KismetArrayLibrary.Array_Length` (`self.Waypoints`)) 1))
        (set `self.CurrentWaypoints` 0)
        (`self.EnemyMoveTo1`)
        (else
          (`/Engine/EditorBlueprintResources/StandardMacros.IncrementInt` (`self.CurrentWaypoints`)
            (:`  `
              (`self.EnemyMoveTo1`))))))))

(event `EnemyMoveTo3`
  (`|AIMoveTo` self (0.0 0.0 0.0) (`|GetArrayItem` (`self.Waypoints`) (`self.CurrentWaypoints`))
    (:`OnSuccess`
      (if (>= (`self.CurrentWaypoints`) (- (`KismetArrayLibrary.Array_Length` (`self.Waypoints`)) 1))
        (set `self.CurrentWaypoints` 0)
        (`self.EnemyMoveTo1`)
        (else
          (`/Engine/EditorBlueprintResources/StandardMacros.IncrementInt` (`self.CurrentWaypoints`)
            (:`  `
              (`self.EnemyMoveTo1`))))))))

(event `self.ReceiveBeginPlay`
  (bind _asbp_master_vehicle (cast `/Game/Vehicles/MasterVehicle/BP_MasterVehicle` (`GameplayStatics.GetPlayerPawn` 0)))
  (set `self.BPREF_MasterVehicle` _asbp_master_vehicle))

(event `EVNT_OnDeath`
  (bind _bpref_mastervehicle (`self.BPREF_MasterVehicle`))
  (bind _bpref_mastervehicle_2 (`self.BPREF_MasterVehicle`))
  (set `/Game/Vehicles/MasterVehicle/BP_MasterVehicle.Score` (+ (`/Game/Vehicles/MasterVehicle/BP_MasterVehicle.Score` _bpref_mastervehicle_2) (`self.Points`)) _bpref_mastervehicle_2)
  (set `/Game/Vehicles/MasterVehicle/BP_MasterVehicle.Currency` (+ (`/Game/Vehicles/MasterVehicle/BP_MasterVehicle.Currency` _bpref_mastervehicle) (`self.CurrencyPoints`)) _bpref_mastervehicle)
  (`/Game/Vehicles/MasterVehicle/BP_MasterVehicle.EVNT_BoostRefill` (`self.BPREF_MasterVehicle`))
  (`self.K2_DestroyActor`))

(event `self.ReceiveTick`
  (params (DeltaSeconds :type "Float (single-precision)"))
  (`KismetSystemLibrary.PrintString` (`KismetStringLibrary.Concat_StrStr` "Health: " (`KismetStringLibrary.Conv_IntToString` (`self.Health`))) true true (struct :`G` 0.66 :`B` 1.0 :`A` 1.0) 0.0)
  (if (<= (`self.Health`) 0)
    (`self.K2_DestroyActor`)))

(event `self.CapsuleComponent.OnComponentBeginOverlap`
  (params (OverlappedComponent :type "PrimitiveComponent Object Reference") (OtherActor :type "Actor Object Reference") (OtherComp :type "PrimitiveComponent Object Reference") (OtherBodyIndex :type Integer) (bFromSweep :type Boolean) (SweepResult :type "HitResult Structure (by ref)"))
  (bind _body (`/Game/Vehicles/MasterVehicle/BP_MasterVehicle.Body` (`self.BPREF_MasterVehicle`)))
  (if (`self.ActorHasTag` OtherActor "Vehicle")
    (bind _returnvalue (`PrimitiveComponent.GetPhysicsLinearVelocity` _body "None"))
    (`PrimitiveComponent.SetPhysicsLinearVelocity` _body (* _returnvalue (`self.SpeedReductionFactor`)) false "None")
    (`self.EVNT_OnDeath`)))

(fn `UserConstructionScript`)