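; BP_Ennemy_Wave is a wave enemy that patrols an ordered list of waypoint actors in an endless loop.
; The EnemyMoveTo event runs AIMoveTo toward the current waypoint, then on success advances the index, wrapping to zero after the last, and calls itself again.
; Nothing in this graph starts the patrol or handles a failed move, and BeginPlay, overlap and Tick are disabled stubs.
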(event `EnemyMoveTo`
  (`|AIMoveTo` self (0.0 0.0 0.0) (`|GetArrayItem` (`self.Waypoints`) (`self.CurrentWaypoints`))
    (:`OnSuccess`
      (if (>= (`self.CurrentWaypoints`) (- (`KismetArrayLibrary.Array_Length` (`self.Waypoints`)) 1))
        (set `self.CurrentWaypoints` 0)
        (`self.EnemyMoveTo`)
        (else
          (`/Engine/EditorBlueprintResources/StandardMacros.IncrementInt` (`self.CurrentWaypoints`)
            (:`  `
              (`self.EnemyMoveTo`))))))))

(fn `UserConstructionScript`
  (`parent.UserConstructionScript`))