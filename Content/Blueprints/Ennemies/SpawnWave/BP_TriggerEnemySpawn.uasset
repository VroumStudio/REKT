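; Trigger volume that spawns a wave of three enemy types in SpawnArea when the player's vehicle enters it.
; On BeginPlay it caches the player vehicle and gathers blue, green and yellow waypoint actors, one set per type.
; Overlap fires a beacon and a timeline driving the post-process spawn pulse.
; The timeline's Update also runs the spawn loops, handing each enemy its waypoints and starting its movement.
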(event `self.ReceiveBeginPlay`
  (bind _asbp_master_vehicle (cast `/Game/Vehicles/MasterVehicle/BP_MasterVehicle` (`GameplayStatics.GetPlayerPawn` 0)))
  (set `self.BPREF_masterVehicle` _asbp_master_vehicle)
  ;[1 1 1] Set the waypoints for each Ennemy Class
  (bind _outactors (`GameplayStatics.GetAllActorsOfClass` "/Game/Blueprints/Ennemies/SpawnWave/BP_WaypointsBlue.BP_WaypointsBlue_C"))
  (for _array_element _outactors
    (`KismetArrayLibrary.Array_Add` (`self.Waypoints1`) _array_element))
  (bind _outactors_2 (`GameplayStatics.GetAllActorsOfClass` "/Game/Blueprints/Ennemies/SpawnWave/BP_WaypointsGreen.BP_WaypointsGreen_C"))
  (for _array_element_2 _outactors_2
    (`KismetArrayLibrary.Array_Add` (`self.Waypoints2`) _array_element_2))
  (bind _outactors_3 (`GameplayStatics.GetAllActorsOfClass` "/Game/Blueprints/Ennemies/SpawnWave/BP_WaypointsYellow.BP_WaypointsYellow_C"))
  (for _array_element_3 _outactors_3
    (`KismetArrayLibrary.Array_Add` (`self.Waypoints3`) _array_element_3)))

(event `self.SpawnTrigger.OnComponentBeginOverlap`
  (params (OverlappedComponent :type "PrimitiveComponent Object Reference") (OtherActor :type "Actor Object Reference") (OtherComp :type "PrimitiveComponent Object Reference") (OtherBodyIndex :type Integer) (bFromSweep :type Boolean) (SweepResult :type "HitResult Structure (by ref)"))
  (bind _returnvalue (`SceneComponent.K2_GetComponentLocation` (`self.SpawnArea`)))
  (bind _dmi_carpostprocess (`/Game/Vehicles/MasterVehicle/BP_MasterVehicle.DMI_CarPostProcess` (`self.BPREF_masterVehicle`)))
  (if (`self.ActorHasTag` OtherActor "Vehicle")
    (`KismetMaterialLibrary.SetVectorParameterValue` "/Game/Materials/Post_Press_Matrials/Radial_Blur_Post_Process/MPC_Sobel_Post_Process.MPC_Sobel_Post_Process" "Enemy_Spawn_Location" (`KismetMathLibrary.Conv_VectorToLinearColor` _returnvalue))
    (`GameplayStatics.SpawnEmitterAtLocation` "/Game/FX/Enemy_SPawn/PS_Enemy_Beacon.PS_Enemy_Beacon" _returnvalue)
    (bind (_direction _alpha_sphere_factor _alpha_between_positions) (`Timeline|Spawn_FX`)
      (:`Update`
        (`MaterialInstanceDynamic.SetScalarParameterValue` _dmi_carpostprocess "Enemy_Spawn_Radius" _alpha_between_positions)
        (`MaterialInstanceDynamic.SetScalarParameterValue` _dmi_carpostprocess "Alpha_Sphere_Mask_Factor" _alpha_sphere_factor)
        (`|ExecutionSequence`
          (:`then_0`
            ;[1 1 1] Spawn the ennemies in a specific area, with random position
            (for _ (range (+ (`self.NumberOfType01Enemies`) 1))
              (`KismetSystemLibrary.Delay` 0.1)
              (bind _returnvalue_2 (`AIBlueprintHelperLibrary.SpawnAIFromClass` (`self.EnemyType01`) null (`self.RandomSpawnInSpecificArea`)))
              (bind _asbp_master_ennemy (cast `/Game/Blueprints/Ennemies/SpawnWave/BP_MasterEnnemy` _returnvalue_2))
              (set `/Game/Blueprints/Ennemies/SpawnWave/BP_MasterEnnemy.Waypoints` (`self.Waypoints1`) _asbp_master_ennemy)
              (`/Game/Blueprints/Ennemies/SpawnWave/BP_MasterEnnemy.EnemyMoveTo1` _asbp_master_ennemy)))
          (:`then_1`
            (for _ (range (+ (`self.NumberofType02Enemies`) 1))
              (`KismetSystemLibrary.Delay` 0.1)
              (bind _returnvalue_3 (`AIBlueprintHelperLibrary.SpawnAIFromClass` (`self.EnemyType02`) null (`self.RandomSpawnInSpecificArea`)))
              (bind _asbp_master_ennemy_2 (cast `/Game/Blueprints/Ennemies/SpawnWave/BP_MasterEnnemy` _returnvalue_3))
              (set `/Game/Blueprints/Ennemies/SpawnWave/BP_MasterEnnemy.Waypoints` (`self.Waypoints2`) _asbp_master_ennemy_2)
              (`/Game/Blueprints/Ennemies/SpawnWave/BP_MasterEnnemy.EnemyMoveTo2` _asbp_master_ennemy_2)))
          (:`then_2`
            (for _ (range (+ (`self.NumberOfType03Enemies`) 1))
              (`KismetSystemLibrary.Delay` 0.1)
              (bind _returnvalue_4 (`AIBlueprintHelperLibrary.SpawnAIFromClass` (`self.EnemyType03`) null (`self.RandomSpawnInSpecificArea`)))
              (bind _asbp_master_ennemy_3 (cast `/Game/Blueprints/Ennemies/SpawnWave/BP_MasterEnnemy` _returnvalue_4))
              (set `/Game/Blueprints/Ennemies/SpawnWave/BP_MasterEnnemy.Waypoints` (`self.Waypoints3`) _asbp_master_ennemy_3)
              (`/Game/Blueprints/Ennemies/SpawnWave/BP_MasterEnnemy.EnemyMoveTo3` _asbp_master_ennemy_3)))))
      (:`Finished`
        (`MaterialInstanceDynamic.SetScalarParameterValue` _dmi_carpostprocess "Enemy_Spawn_Radius" 0.0)
        (`MaterialInstanceDynamic.SetScalarParameterValue` _dmi_carpostprocess "Alpha_Sphere_Mask_Factor" 0.0)))))

(fn `UserConstructionScript`)