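; Enemy pawn Blueprint that patrols a looping route of waypoint actors.
; The EnemyMoveTo event uses AIMoveTo toward the current waypoint; on success it advances the index, wrapping to the first after the last, and calls itself again.
; Despite the spawning name, the file holds no spawn logic, no caller that starts the patrol, and no handling for failed moves.
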(event `EnemyMoveTo`
  (`|AIMoveTo` self (0.0 0.0 0.0) (`|GetArrayItem` (`self.Waypoints`) (`self.CurrentWaypoint`))
    (:`OnSuccess`
      (if (>= (`self.CurrentWaypoint`) (- (`KismetArrayLibrary.Array_Length` (`self.Waypoints`)) 1))
        (set `self.CurrentWaypoint` 0)
        (`self.EnemyMoveTo`)
        (else
          (`/Engine/EditorBlueprintResources/StandardMacros.IncrementInt` (`self.CurrentWaypoint`)
            (:`  `
              (`self.EnemyMoveTo`))))))))

(fn `UserConstructionScript`)