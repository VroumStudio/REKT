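; Behavior Tree task for the test Runner enemy that sets its next patrol destination from the current Route index.
; It resets Route to zero once it reaches MaxRoutes, but does not increment it.
; It then scans all BP_TargetPoint actors and writes the location of the one whose Position matches Route to the TargetPoint blackboard key.
; After the scan it always finishes as failed.
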(event `self.ReceiveExecuteAI`
  (params (OwnerController :type "AIController Object Reference") (ControlledPawn :type "Pawn Object Reference"))
  (bind _route (`self.Route`))
  (if (>= (`BTFunctionLibrary.GetBlackboardValueAsInt` _route) (`self.MaxRoutes`))
    (`BTFunctionLibrary.SetBlackboardValueAsInt` _route))
  (bind _outactors (`GameplayStatics.GetAllActorsOfClass` "/Game/Blueprints/Ennemies/Test_BT_BB_Runner/BP_TargetPoint.BP_TargetPoint_C"))
  (for _array_element _outactors
    (bind _asbp_target_point (cast `/Game/Blueprints/Ennemies/Test_BT_BB_Runner/BP_TargetPoint` _array_element))
    (if (== (`BTFunctionLibrary.GetBlackboardValueAsInt` (`self.Route`)) (`/Game/Blueprints/Ennemies/Test_BT_BB_Runner/BP_TargetPoint.Position` _asbp_target_point))
      (`BTFunctionLibrary.SetBlackboardValueAsVector` (`self.TargetPoint`) (`Actor.K2_GetActorLocation` _asbp_target_point))))
  (`self.FinishExecute` false))