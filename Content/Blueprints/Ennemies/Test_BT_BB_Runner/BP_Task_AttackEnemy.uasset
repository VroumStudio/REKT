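; Behavior Tree task for the Runner enemy AI, meant to drive its attack on a muscle car target.
; Execute only casts the owner to the Runner controller; the remaining logic is disconnected, so the task never calls FinishExecute.
; That unused logic checks the blackboard EnemyActor and State, calling EnemyFound and failing on Attack, or succeeding on Patrol and Search.
; An invalid target there resets State and calls EnemyLost.
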(event `self.ReceiveExecuteAI`
  (params (OwnerController :type "AIController Object Reference") (ControlledPawn :type "Pawn Object Reference"))
  (bind _asbp_ai_controller_runner (cast `/Game/Blueprints/Ennemies/Test_BT_BB_Runner/BP_AI_Controller_Runner` OwnerController)))