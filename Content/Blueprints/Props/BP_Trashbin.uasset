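; BP_Trashbin is a trash bin prop whose header appearance varies with a TextureSet selection.
; The construction script creates a dynamic instance of MI_TrashbinHeader on element 0 of the static mesh.
; It sets that material's Alpha texture and Color from the selected set, with no texture assigned for TextureSet02.
; The event graph holds only disabled placeholder events, so the Blueprint adds no runtime logic.
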(fn `UserConstructionScript`
  (bind _returnvalue (`PrimitiveComponent.CreateDynamicMaterialInstance` (`self.StaticMesh`) 0 "/Game/Materials/Props/Trashbin/MI_TrashbinHeader.MI_TrashbinHeader" "None"))
  (set `self.DMI_TrashbinHeader` _returnvalue)
  (`MaterialInstanceDynamic.SetTextureParameterValue` (`self.DMI_TrashbinHeader`) "Alpha" (select `/Game/Blueprints/Props/E_TrashbinTextureSet` (`self.TextureSet`) :`NewEnumerator0` "/Game/Textures/Props/Trashbin/T_Trashbin_Header_TextureSet01_O.T_Trashbin_Header_TextureSet01_O" :`NewEnumerator2` "/Game/Textures/Props/Trashbin/T_Trashbin_Header_TextureSet03_O.T_Trashbin_Header_TextureSet03_O" :`NewEnumerator3` "/Game/Textures/Props/Trashbin/T_Trashbin_Header_TextureSet04_O.T_Trashbin_Header_TextureSet04_O" :!type "Texture Object Reference"))
  (`MaterialInstanceDynamic.SetVectorParameterValue` (`self.DMI_TrashbinHeader`) "Color" (select `/Game/Blueprints/Props/E_TrashbinTextureSet` (`self.TextureSet`) :`NewEnumerator0` (struct :`G` 1.0 :`A` 1.0) :`NewEnumerator2` (struct :`B` 1.0 :`A` 1.0) :`NewEnumerator3` (struct :`R` 1.0 :`G` 1.0 :`B` 1.0 :`A` 1.0) :!type "LinearColor Structure")))