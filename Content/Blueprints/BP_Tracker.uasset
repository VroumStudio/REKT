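; BP_Tracker is a checkpoint tracker for a vehicle game, holding the checkpoint count and a reference to the player's vehicle.
; On BeginPlay it casts the player pawn to BP_MasterVehicle, stopping if that fails, then counts all BP_Checkpoint actors in the level.
; PrintDebug prints that count plus the vehicle's last and total crossed checkpoints, though both totals share the same "Total Checkpoints:" label.
; Nothing in this Blueprint calls PrintDebug.
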(event `self.ReceiveBeginPlay`
  (bind _asbp_master_vehicle (cast `/Game/Vehicles/MasterVehicle/BP_MasterVehicle` (`GameplayStatics.GetPlayerPawn` 0)))
  (set `self.BPREF_MasterVehicle` _asbp_master_vehicle)
  (bind _outactors (`GameplayStatics.GetAllActorsOfClass` "/Game/Blueprints/Checkpoints/BP_Checkpoint.BP_Checkpoint_C"))
  (set `self.NumberOfCheckpoints` (`KismetArrayLibrary.Array_Length` _outactors)))

(fn `PrintDebug`
  (params (bPrintToScreen :type Boolean))
  (`KismetSystemLibrary.PrintString` (`KismetStringLibrary.Concat_StrStr` "Total Checkpoints: " (`KismetStringLibrary.Conv_IntToString` (`self.NumberOfCheckpoints`))) bPrintToScreen false (struct :`G` 0.66 :`B` 1.0 :`A` 1.0) 0.0)
  (`KismetSystemLibrary.PrintString` (`KismetStringLibrary.Concat_StrStr` "Last Checkpoint: " (`KismetStringLibrary.Conv_IntToString` (`/Game/Vehicles/MasterVehicle/BP_MasterVehicle.LastCrossedCheckpoint` (`self.BPREF_MasterVehicle`)))) bPrintToScreen false (struct :`G` 0.66 :`B` 1.0 :`A` 1.0) 0.0)
  (`KismetSystemLibrary.PrintString` (`KismetStringLibrary.Concat_StrStr` "Total Checkpoints: " (`KismetStringLibrary.Conv_IntToString` (`/Game/Vehicles/MasterVehicle/BP_MasterVehicle.TotalCrossedCheckpoints` (`self.BPREF_MasterVehicle`)))) bPrintToScreen false (struct :`G` 0.66 :`B` 1.0 :`A` 1.0) 0.0))

(fn `UserConstructionScript`)