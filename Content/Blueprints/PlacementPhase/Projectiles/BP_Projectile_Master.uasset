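; BP_Projectile_Master is a configurable projectile actor in the PlacementPhase folder, named as the master for projectile Blueprints.
; Its construction script feeds speed variables into ProjectileMovement, applies the chosen static mesh and replaces the actor's Tags with UserTags.
; It also assigns Damages to itself, with no damage logic here.
; The event graph holds only disabled placeholder events, so no runtime behavior is scripted in this Blueprint.
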(fn `UserConstructionScript`
  (bind _projectilemovement (`self.ProjectileMovement`))
  (set `ProjectileMovementComponent.InitialSpeed` (`self.InitialSpeed`) _projectilemovement)
  (set `ProjectileMovementComponent.MaxSpeed` (`self.MaxSpeed`) _projectilemovement)
  (`StaticMeshComponent.SetStaticMesh` (`self.StaticMesh`) (`self.ProjectileMesh`))
  (set `self.Damages` (`self.Damages`))
  (set `self.Tags` (`|MakeArray` (`self.UserTags`))))