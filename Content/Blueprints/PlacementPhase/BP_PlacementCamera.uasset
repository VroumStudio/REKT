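; Placement-phase camera actor that shows the mouse cursor and pans based on its screen position.
; Each Tick compares cursor X and Y to hard-coded pixel thresholds and derives a speed from the pixel distance.
; Horizontal speed offsets the actor along the camera's right vector, including between the two thresholds, but not beyond the upper one.
; The vertical branch computes a speed but applies a zero offset, so it produces no movement.
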(event `self.ReceiveBeginPlay`
  (set `PlayerController.bShowMouseCursor` true (`GameplayStatics.GetPlayerController` 0)))

(event `self.ReceiveTick`
  (params (DeltaSeconds :type "Float (single-precision)"))
  (bind (_locationx _locationy) (`PlayerController.GetMousePosition` (`GameplayStatics.GetPlayerController` 0)))
  (if (< _locationx 300.0)
    (set `self.MouvementSpeed` (/ (- _locationx 300.0) 15.0))
    (`self.K2_AddActorWorldOffset` (* (`SceneComponent.GetRightVector` (`self.Camera`)) (`self.MouvementSpeed`)) :!label _label)
    (elif (< _locationx 1620.0)
      (set `self.MouvementSpeed` (/ (- _locationx 1620.0) 15.0))
      (goto _label)
      (else
        _)))
  (if (< _locationy 150.0)
    (set `self.MouvementSpeed` (/ (- _locationy 300.0) 15.0))
    (`self.K2_AddActorWorldOffset` (0.0 0.0 0.0) :!label _label_2)
    (elif (< _locationy 930.0)
      (set `self.MouvementSpeed` (/ (- _locationy 1620.0) 15.0))
      (goto _label_2))))

(fn `UserConstructionScript`)