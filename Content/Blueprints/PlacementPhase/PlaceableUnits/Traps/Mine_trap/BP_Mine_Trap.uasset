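; Mine trap actor for the placement phase, handling the trap's animation, warning glow and removal.
; On spawn it creates a dynamic emissive material and drives its opacity with the Opacity_Warning timeline.
; Collision box overlaps toggle IsTriggered on the anim Blueprint.
; Any begin overlap also lights the emissive fully, then turns it off and destroys the actor after short delays; no damage is applied here.
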(event `self.ReceiveBeginPlay`
  (bind _returnvalue (`PrimitiveComponent.CreateDynamicMaterialInstance` (`self.Mine_Trap_LOW_Rigged`) 1 "/Game/Blueprints/PlacementPhase/PlaceableUnits/Traps/Mine_trap/M_Emissive_Mine_Trap_Instance.M_Emissive_Mine_Trap_Instance" "None"))
  (set `self.Mine_Emissive_Instance` _returnvalue)
  (bind _asabp_trap_mine (cast `/Game/Blueprints/PlacementPhase/PlaceableUnits/Traps/Mine_trap/Anims/ABP_Trap_Mine` (`SkeletalMeshComponent.GetAnimInstance` (`self.Mine_Trap_LOW_Rigged`))))
  (set `self.MineTrap_Anim_BP` _asabp_trap_mine)
  (bind (_direction _opacity_track) (`Timeline|Opacity_Warning`)
    (:`Update`
      (`MaterialInstanceDynamic.SetScalarParameterValue` (`self.Mine_Emissive_Instance`) "Opacity" _opacity_track))))

(event `self.Collision_Box.OnComponentBeginOverlap`
  (params (OverlappedComponent :type "PrimitiveComponent Object Reference") (OtherActor :type "Actor Object Reference") (OtherComp :type "PrimitiveComponent Object Reference") (OtherBodyIndex :type Integer) (bFromSweep :type Boolean) (SweepResult :type "HitResult Structure (by ref)"))
  (set `/Game/Blueprints/PlacementPhase/PlaceableUnits/Traps/Mine_trap/Anims/ABP_Trap_Mine.Is Triggered` true (`self.MineTrap_Anim_BP`))
  (`|ExecutionSequence`
    (:`then_1`
      (`MaterialInstanceDynamic.SetScalarParameterValue` (`self.Mine_Emissive_Instance`) "Opacity" 1.0)
      (`KismetSystemLibrary.Delay` 2.0)
      (`MaterialInstanceDynamic.SetScalarParameterValue` (`self.Mine_Emissive_Instance`) "Opacity" 0.0)
      (`KismetSystemLibrary.Delay` 1.0)
      (`self.K2_DestroyActor`))))

(event `self.Collision_Box.OnComponentEndOverlap`
  (params (OverlappedComponent :type "PrimitiveComponent Object Reference") (OtherActor :type "Actor Object Reference") (OtherComp :type "PrimitiveComponent Object Reference") (OtherBodyIndex :type Integer))
  (set `/Game/Blueprints/PlacementPhase/PlaceableUnits/Traps/Mine_trap/Anims/ABP_Trap_Mine.Is Triggered` false (`self.MineTrap_Anim_BP`)))

(fn `UserConstructionScript`)