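; Gatling turret Blueprint, a placeable unit that fires at actors entering its Range component.
; On BeginPlay it caches its skeletal mesh's ABP_Turret_Gatling anim instance, which holds the targeting state.
; Range overlap begin and end toggle CanShoot on that instance, with no actor filtering.
; Tick copies the overlapping actor into the instance's TargetActor and calls Fire while CanShoot is true.
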(event `self.ReceiveBeginPlay`
  (`parent.ReceiveBeginPlay`)
  (bind _asabp_turret_gatling (cast `/Game/Blueprints/PlacementPhase/PlaceableUnits/Turrets/Gatling_Turret/Animation/ABP_Turret_Gatling` (`SkeletalMeshComponent.GetAnimInstance` (`self.SkeletalMesh`))))
  (set `self.ABPREF_Turret_Gatling` _asabp_turret_gatling))

(event `self.ReceiveTick`
  (params (DeltaSeconds :type "Float (single-precision)"))
  (bind _abpref_turret_gatling (`self.ABPREF_Turret_Gatling`))
  (set `/Game/Blueprints/PlacementPhase/PlaceableUnits/Turrets/Gatling_Turret/Animation/ABP_Turret_Gatling.TargetActor` (stale `self.Range.OnComponentBeginOverlap` OtherActor) _abpref_turret_gatling)
  (if (`/Game/Blueprints/PlacementPhase/PlaceableUnits/Turrets/Gatling_Turret/Animation/ABP_Turret_Gatling.Can_Shoot` _abpref_turret_gatling)
    (`self.Fire`)))

(event `self.Range.OnComponentBeginOverlap`
  (params (OverlappedComponent :type "PrimitiveComponent Object Reference") (OtherActor :type "Actor Object Reference") (OtherComp :type "PrimitiveComponent Object Reference") (OtherBodyIndex :type Integer) (bFromSweep :type Boolean) (SweepResult :type "HitResult Structure (by ref)"))
  (set `/Game/Blueprints/PlacementPhase/PlaceableUnits/Turrets/Gatling_Turret/Animation/ABP_Turret_Gatling.Can_Shoot` true (`self.ABPREF_Turret_Gatling`)))

(event `self.Range.OnComponentEndOverlap`
  (params (OverlappedComponent :type "PrimitiveComponent Object Reference") (OtherActor :type "Actor Object Reference") (OtherComp :type "PrimitiveComponent Object Reference") (OtherBodyIndex :type Integer))
  (set `/Game/Blueprints/PlacementPhase/PlaceableUnits/Turrets/Gatling_Turret/Animation/ABP_Turret_Gatling.Can_Shoot` false (`self.ABPREF_Turret_Gatling`)))

(fn `UserConstructionScript`
  (`parent.UserConstructionScript`))