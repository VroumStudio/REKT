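; Master turret Blueprint for a placeable unit that detects enemies and fires projectiles.
; The construction script applies the mesh and animation Blueprint and sizes the Range capsule from Size.
; Range overlaps set LockedTarget for tagged actors and clear it when any actor leaves.
; Fire, not called here, waits on FireRate, then spawns a hardcoded BP_Projectile_Master at the cannon socket; the placement-point cost check is unwired.
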(event `self.ReceiveBeginPlay`
  (bind _asbp_menu_pawn (cast `/Game/Blueprints/Base/BP_MenuPawn` (`GameplayStatics.GetPlayerPawn` 0)))
  (set `self.BPREF_Pawn` _asbp_menu_pawn)
  (set `self.Cost` (`self.Cost`)))

(event `self.Range.OnComponentBeginOverlap`
  (params (OverlappedComponent :type "PrimitiveComponent Object Reference") (OtherActor :type "Actor Object Reference") (OtherComp :type "PrimitiveComponent Object Reference") (OtherBodyIndex :type Integer) (bFromSweep :type Boolean) (SweepResult :type "HitResult Structure (by ref)"))
  (if (or (`self.ActorHasTag` OtherActor "Ennemy") (`self.ActorHasTag` OtherActor "Targetable"))
    (set `self.bLockedTarget` true)))

(event `self.Range.OnComponentEndOverlap`
  (params (OverlappedComponent :type "PrimitiveComponent Object Reference") (OtherActor :type "Actor Object Reference") (OtherComp :type "PrimitiveComponent Object Reference") (OtherBodyIndex :type Integer))
  (set `self.bLockedTarget` false))

(event `Fire`
  (bind (_returnvalue_location _returnvalue_rotation) (`KismetMathLibrary.BreakTransform` (`SceneComponent.GetSocketTransform` (`self.SkeletalMesh`) "Socket_Cannon" "RTS_World")))
  (`KismetSystemLibrary.Delay` (/ (`self.FireRate`) 60.0))
  (`|SpawnActorFromClass` "/Game/Blueprints/PlacementPhase/Projectiles/BP_Projectile_Master.BP_Projectile_Master_C" (`KismetMathLibrary.MakeTransform` _returnvalue_location _returnvalue_rotation (0.2 0.2 0.2)) "Undefined" "OverrideRootScale" null 1500.0 1500.0 "/Engine/EditorMeshes/ArcadeEditorSphere.ArcadeEditorSphere" "Projectile" null))

(fn `UserConstructionScript`
  (bind _range (`self.Range`))
  (bind _truesize (`self.TrueSize`))
  (bind _skeletalmesh (`self.SkeletalMesh`))
  (`SkinnedMeshComponent.SetSkinnedAssetAndUpdate` _skeletalmesh (`self.TurretMesh`) true)
  (`SkeletalMeshComponent.K2_SetAnimInstanceClass` _skeletalmesh (`self.AnimationBlueprint`))
  (set `self.ProjectileClass` (`self.ProjectileClass`))
  (set `self.TrueSize` (* (`self.Size`) 100.0))
  (`CapsuleComponent.SetCapsuleRadius` _range _truesize true)
  (`CapsuleComponent.SetCapsuleHalfHeight` _range _truesize true))