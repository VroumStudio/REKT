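; BP_Gatling is a placeable gatling turret unit that tracks and fires at actors entering its Range.
; The latest overlap becomes Target, and any exit clears the lock.
; While locked, Tick aims horizontal and vertical PoseableMesh bones and calls Fire, whose Delay throttles projectile spawns at a fixed world location, unrotated.
; BeginPlay caches the aerial player pawn, but the placement-points cost check is left unwired.
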(event `self.ReceiveBeginPlay`
  (bind _asbp_aerial_pawn (cast `/Game/Blueprints/Base/BP_AerialPawn` (`GameplayStatics.GetPlayerPawn` 0)))
  (set `self.BPREF_Pawn` _asbp_aerial_pawn)
  (set `self.Cost` (`self.Cost`)))

(event `UpdateTurretRotation`
  (bind _poseablemesh (`self.PoseableMesh`))
  (bind _returnvalue (`SceneComponent.K2_GetComponentLocation` _poseablemesh))
  (bind _x (.x (`self.K2_GetActorLocation` (`self.Target`))))
  (bind _y (.y (`self.K2_GetActorLocation` (`self.Target`))))
  (`|ExecutionSequence`
    (:`then_0`
      (`PoseableMeshComponent.SetBoneRotationByName` _poseablemesh "Horizontal_Rotator" (`KismetMathLibrary.FindLookAtRotation` _returnvalue (`KismetMathLibrary.MakeVector` _x _y)) "WorldSpace"))
    (:`then_1`
      (`PoseableMeshComponent.SetBoneRotationByName` _poseablemesh "Vertical_Rotator" (`KismetMathLibrary.FindLookAtRotation` _returnvalue (`KismetMathLibrary.MakeVector` _x _y (- (.z (`self.K2_GetActorLocation` (`self.Target`))) 200.0))) "WorldSpace"))))

(event `self.Range.OnComponentBeginOverlap`
  (params (OverlappedComponent :type "PrimitiveComponent Object Reference") (OtherActor :type "Actor Object Reference") (OtherComp :type "PrimitiveComponent Object Reference") (OtherBodyIndex :type Integer) (bFromSweep :type Boolean) (SweepResult :type "HitResult Structure (by ref)"))
  (set `self.bLockedTarget` true)
  (set `self.Target` OtherActor))

(event `self.Range.OnComponentEndOverlap`
  (params (OverlappedComponent :type "PrimitiveComponent Object Reference") (OtherActor :type "Actor Object Reference") (OtherComp :type "PrimitiveComponent Object Reference") (OtherBodyIndex :type Integer))
  (set `self.bLockedTarget` false))

(event `self.ReceiveTick`
  (params (DeltaSeconds :type "Float (single-precision)"))
  (if (`self.bLockedTarget`)
    (`self.UpdateTurretRotation`)
    (`self.Fire`)))

(event `Fire`
  (`KismetSystemLibrary.Delay` (/ (`self.FireRate`) 60.0))
  (`|SpawnActorFromClass` (`self.ProjectileClass`) (`KismetMathLibrary.MakeTransform` (0.0 0.0 400.0)) "Undefined" "OverrideRootScale" null null))

(fn `UserConstructionScript`
  (`SkinnedMeshComponent.SetSkinnedAssetAndUpdate` (`self.PoseableMesh`) (`self.TurretMesh`) true)
  (set `self.ProjectileClass` (`self.ProjectileClass`)))