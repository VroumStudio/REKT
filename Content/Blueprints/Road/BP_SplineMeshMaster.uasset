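; Road spline Blueprint that builds a chain of deformed mesh segments with collision along its spline.
; The construction script divides spline length by Spacing and adds a manually attached spline mesh component per step, using the configurable Mesh.
; World-space positions and TangentScale-scaled directions at each distance shape the segments.
; Start and end roll share one value, read by spline point index equal to the segment index rather than by distance.
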(fn `UserConstructionScript`
  (bind _spline (`self.Spline`))
  (bind _spacing (`self.Spacing`))
  (for _index (range (+ (`.ReturnValue` (`KismetMathLibrary.FMod` (`SplineComponent.GetSplineLength` _spline) _spacing)) 1))
    (bind _returnvalue (`AddComponent|NODE_AddSplineMeshComponent-1` :`bManualAttachment` true))
    (`StaticMeshComponent.SetStaticMesh` _returnvalue (`self.Mesh`))
    (bind _returnvalue_2 (* _index _spacing))
    (bind _returnvalue_3 (+ _returnvalue_2 _spacing))
    (`SplineMeshComponent.SetStartAndEnd` _returnvalue (`SplineComponent.GetLocationAtDistanceAlongSpline` _spline _returnvalue_2 "World") (* (`SplineComponent.GetDirectionAtDistanceAlongSpline` _spline _returnvalue_2 "World") (`self.TangentScale`)) (`SplineComponent.GetLocationAtDistanceAlongSpline` _spline _returnvalue_3 "World") (* (`SplineComponent.GetDirectionAtDistanceAlongSpline` _spline _returnvalue_3 "World") (`self.TangentScale`)) true)
    (bind _returnvalue_4 (`SplineComponent.GetRollAtSplinePoint` _spline _index "World"))
    (`SplineMeshComponent.SetStartRoll` _returnvalue _returnvalue_4 true)
    (`SplineMeshComponent.SetEndRoll` _returnvalue _returnvalue_4 true)
    (`PrimitiveComponent.SetCollisionEnabled` _returnvalue "QueryAndPhysics")))