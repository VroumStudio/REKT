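; BP_SplineMaster is a road spline Blueprint that lays a chosen mesh along a spline.
; Its construction script divides the spline length by Spacing and creates a manually attached spline mesh component for each segment.
; Each segment takes world-space start and end positions, scaled direction tangents and roll from the spline at those distances, so the mesh follows its curves and banking.
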(fn `UserConstructionScript`
  (bind _splinemesh (`self.SplineMesh`))
  (bind _spacing (`self.Spacing`))
  (for _index (range (+ (`.ReturnValue` (`KismetMathLibrary.FMod` (`SplineComponent.GetSplineLength` (`self.Spline`)) (`self.Spacing`))) 1))
    (bind _returnvalue (`AddComponent|NODE_AddSplineMeshComponent-4` :`bManualAttachment` true))
    (bind _output_get (set `self.SplineMesh` _returnvalue))
    (`StaticMeshComponent.SetStaticMesh` _output_get (`self.Mesh`))
    (bind _returnvalue_2 (* _index _spacing))
    (bind _returnvalue_3 (+ _returnvalue_2 _spacing))
    (`SplineMeshComponent.SetStartAndEnd` (`self.SplineMesh`) (`SplineComponent.GetLocationAtDistanceAlongSpline` (`self.Spline`) _returnvalue_2 "World") (* (`SplineComponent.GetDirectionAtDistanceAlongSpline` (`self.Spline`) _returnvalue_2 "World") (`self.Tangent`)) (`SplineComponent.GetLocationAtDistanceAlongSpline` (`self.Spline`) _returnvalue_3 "World") (* (`SplineComponent.GetDirectionAtDistanceAlongSpline` (`self.Spline`) _returnvalue_3 "World") (`self.Tangent`)) true)
    (`SplineMeshComponent.SetStartRoll` _splinemesh (`KismetMathLibrary.DegreesToRadians` (.roll (`SplineComponent.GetRotationAtDistanceAlongSpline` (`self.Spline`) _returnvalue_2 "World"))) true)
    (`SplineMeshComponent.SetEndRoll` _splinemesh (`KismetMathLibrary.DegreesToRadians` (.roll (`SplineComponent.GetRotationAtDistanceAlongSpline` (`self.Spline`) _returnvalue_3 "World"))) true)))