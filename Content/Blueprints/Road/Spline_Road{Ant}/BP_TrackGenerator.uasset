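; BP_TrackGenerator builds a looping road track along its spline in the construction script.
; It caches the spline point count and resizes RoadDataArray to match, one entry per point.
; BuildTrackElement then adds a RoadMesh spline mesh per point, shaped by local-space locations and tangents, with modulo indexing joining last to first.
; RoadDataArray is not yet used in building; its Left_Guard_Rail read is unconnected.
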(fn `Build_Track_Element`
  (params (Loop_Index :type Integer) (Track_Element_Mesh :type "StaticMesh Object Reference"))
  (locals (Local_Current_Loop_Index :type Integer) (Local_Next_Loop_Index :type Integer) (Local_Track_Element_Mesh :type "StaticMesh Object Reference") (Local_Start_Location :type "Vector Structure" :default (1.0 0.0 0.0)) (Local_Start_Tangent :type "Vector Structure" :default (1.0 0.0 0.0)) (Local_End_Location :type "Vector Structure" :default (1.0 0.0 0.0)) (Local_End_Tangent :type "Vector Structure" :default (1.0 0.0 0.0)) (Local_Current_Spline_Mesh :type "SplineMeshComponent Object Reference") (Local_Start_Roll :type "Float (double-precision)"))
  (bind (_location _tangent) (`SplineComponent.GetLocationAndTangentAtSplinePoint` (`self.Spline`) (`local.Local_Next_Loop_Index`) "Local"))
  (bind (_location_2 _tangent_2) (`SplineComponent.GetLocationAndTangentAtSplinePoint` (`self.Spline`) (`local.Local_Current_Loop_Index`) "Local"))
  (set `local.Local_Current_Loop_Index` Loop_Index)
  (set `local.Local_Next_Loop_Index` (mod (+ Loop_Index 1) (`self.Number_Of_Spline_Points`)))
  (set `local.Local_Track_Element_Mesh` Track_Element_Mesh)
  (`|ExecutionSequence`
    (:`then_0`
      (set `local.Local_Start_Location` _location_2)
      (set `local.Local_Start_Tangent` _tangent_2)
      (set `local.Local_End_Location` _location)
      (set `local.Local_End_Tangent` _tangent))
    (:`then_1`
      (bind _returnvalue (`AddComponent|NODE_AddSplineMeshComponent-0`))
      (set `local.Local_Current_Spline_Mesh` _returnvalue)
      (`StaticMeshComponent.SetStaticMesh` (`local.Local_Current_Spline_Mesh`) (`local.Local_Track_Element_Mesh`))
      (`SplineMeshComponent.SetStartAndEnd` (`local.Local_Current_Spline_Mesh`) (`local.Local_Start_Location`) (`local.Local_Start_Tangent`) (`local.Local_End_Location`) (`local.Local_End_Tangent`) true))))

(fn `UserConstructionScript`
  (bind _road_data_array (`self.Road_Data_Array`))
  (`|ExecutionSequence`
    (:`then_0`
      (set `self.Number_Of_Spline_Points` (`SplineComponent.GetNumberOfSplinePoints` (`self.Spline`))))
    (:`then_1`
      (`/Engine/EditorBlueprintResources/StandardMacros.CompareInt` (`KismetArrayLibrary.Array_Length` (`self.Road_Data_Array`)) (`self.Number_Of_Spline_Points`) :!label _label
        (:`>`
          (`KismetArrayLibrary.Array_Remove` _road_data_array (`KismetArrayLibrary.Array_LastIndex` _road_data_array))
          (goto _label))
        (:`<`
          (`KismetArrayLibrary.Array_Add` (`self.Road_Data_Array`))
          (goto _label))))
    (:`then_2`
      (for _index (range (`self.Number_Of_Spline_Points`))
        (`self.Build_Track_Element` _index (`self.Road_Mesh`))))
    (:`then_3`)))