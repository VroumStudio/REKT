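; Highway road connector Blueprint without a separator that spawns spline-based road actors at its connection sockets.
; SpawnRoad places a BP_SplineMaster at the chosen socket's location and rotation on the Connector mesh and assigns it the highway road mesh.
; Two events trigger it, one for the selected Socket and one for both connectors in sequence.
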(event `SpawnRoadToSelectedConnector`
  (`self.SpawnRoad` (`self.Socket`)))

(event `SpawnRoadToAllConnectors`
  (`|ExecutionSequence`
    (:`then_0`
      (`self.SpawnRoad` "NewEnumerator0"))
    (:`then_1`
      (`self.SpawnRoad` "NewEnumerator1"))))

(fn `SpawnRoad`
  (params (Socket :type "/Game/Blueprints/Splines/Enumerators/E_Socket_4Ways Enum" :default "NewEnumerator0"))
  (bind _connector (`self.Connector`))
  (bind _connector_2 (`self.Connector`))
  (switch `/Game/Blueprints/Splines/Enumerators/E_Socket_4Ways` Socket
    (:`NewEnumerator0`
      (bind _returnvalue (`|SpawnActorFromClass` "/Game/Blueprints/Splines/BP_SplineMaster.BP_SplineMaster_C" (`KismetMathLibrary.MakeTransform` (`SceneComponent.GetSocketLocation` _connector "Connector1") (`SceneComponent.GetSocketRotation` _connector "Connector1")) "AlwaysSpawn" "OverrideRootScale" null null))
      (set `/Game/Blueprints/Splines/BP_SplineMaster.Mesh` "/Game/Mesh/Roads/SM_Road_Highway.SM_Road_Highway" _returnvalue))
    (:`NewEnumerator1`
      (bind _returnvalue_2 (`|SpawnActorFromClass` "/Game/Blueprints/Splines/BP_SplineMaster.BP_SplineMaster_C" (`KismetMathLibrary.MakeTransform` (`SceneComponent.GetSocketLocation` _connector_2 "Connector2") (`SceneComponent.GetSocketRotation` _connector_2 "Connector2")) "AlwaysSpawn" "OverrideRootScale" null null))
      (set `/Game/Blueprints/Splines/BP_SplineMaster.Mesh` "/Game/Mesh/Roads/SM_Road_Highway.SM_Road_Highway" _returnvalue_2))))

(fn `UserConstructionScript`)