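; BP_SplineMeshMaster is a modular spline mesh actor that lays a configurable static mesh along an editable spline.
; Its construction script adds one spline mesh component per segment between neighbouring spline points, setting its mesh and forward axis and attaching it to the root.
; Each segment bends to the local positions and tangents of its two end points, and the event graph holds no logic.
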(fn `UserConstructionScript`
  (for _index (range (+ (- (`SplineComponent.GetNumberOfSplinePoints` (`self.Spline`)) 2) 1))
    (bind _returnvalue (`AddComponent|NODE_AddSplineMeshComponent-0`))
    (set `self.REF_SplineMeshComp` _returnvalue)
    (`SplineMeshComponent.SetForwardAxis` (`self.REF_SplineMeshComp`) (`self.ForwardAxis`) true)
    (`StaticMeshComponent.SetStaticMesh` (`self.REF_SplineMeshComp`) (`self.Mesh`))
    (`SceneComponent.K2_AttachToComponent` (`self.REF_SplineMeshComp`) (`self.DefaultSceneRoot`) "None" "KeepRelative" "KeepRelative" "KeepRelative" true)
    (bind (_location _tangent) (`SplineComponent.GetLocationAndTangentAtSplinePoint` (`self.Spline`) _index "Local"))
    (bind (_location_2 _tangent_2) (`SplineComponent.GetLocationAndTangentAtSplinePoint` (`self.Spline`) (+ _index 1) "Local"))
    (`SplineMeshComponent.SetStartAndEnd` (`self.REF_SplineMeshComp`) _location _tangent _location_2 _tangent_2 true)))