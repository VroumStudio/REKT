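; BP_Tracker is a checkpoint and lap tracker that holds race data and shows it as on-screen debug text.
; Its construction script gathers all BP_Checkpoint actors into a unique list and stores their count.
; BeginPlay caches the player pawn as a BP_MasterVehicle reference.
; Every Tick prints the remaining laps and that vehicle's last crossed checkpoint; nothing here updates the lap value.
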(event `self.ReceiveBeginPlay`
  (bind _asbp_master_vehicle (cast `/Game/Vehicles/MasterVehicle/BP_MasterVehicle` (`GameplayStatics.GetPlayerPawn` 0)))
  (set `self.BPREF_MuscleCar` _asbp_master_vehicle))

(event `self.ReceiveTick`
  (params (DeltaSeconds :type "Float (single-precision)"))
  (`self.DisplayDebugPrints`))

(fn `DisplayDebugPrints`
  (`KismetSystemLibrary.PrintString` (`KismetStringLibrary.Concat_StrStr` "Lap Remaining: " (`KismetStringLibrary.Conv_IntToString` (`self.Laps`))) true true (struct :`G` 0.66 :`B` 1.0 :`A` 1.0) 0.0)
  (`KismetSystemLibrary.PrintString` (`KismetStringLibrary.Concat_StrStr` "Last Crossed Checkpoint: " (`KismetStringLibrary.Conv_IntToString` (`/Game/Vehicles/MasterVehicle/BP_MasterVehicle.LastCrossedCheckpoint` (`self.BPREF_MuscleCar`)))) true true (struct :`R` 1.0 :`B` 0.040533 :`A` 1.0) 0.0))

(fn `UserConstructionScript`
  (bind _outactors (`GameplayStatics.GetAllActorsOfClass` "/Game/Blueprints/Checkpoints/BP_Checkpoint.BP_Checkpoint_C"))
  (bind _returnvalue (`KismetArrayLibrary.Array_Length` _outactors))
  (for _index (range _returnvalue)
    (`KismetArrayLibrary.Array_AddUnique` (`self.Checkpoints`) (`|GetArrayItem` _outactors _index)))
  (set `self.NumberOfCheckpoints` _returnvalue))