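; Race checkpoint gate that tracks the player vehicle's progress, recoloring its pillars, setting the respawn point and refilling boost.
; On trigger exit it checks crossing direction, then lap and race completion against BP_Tracker, resetting all checkpoints each lap.
; Enemies crossing checkpoint zero cost score.
; Race end fades out, scores time and currency, shows medal and stats, and saves a fresh save object to the level's slot.
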(event `self.ReceiveBeginPlay`
  (bind _asbp_master_vehicle (cast `/Game/Vehicles/MasterVehicle/BP_MasterVehicle` (`GameplayStatics.GetPlayerPawn` 0)))
  (set `self.BPREF_MasterVehicle` _asbp_master_vehicle)
  (bind _asbp_rektgame_mode (cast `/Game/Blueprints/Base/BP_REKTGameMode` (`GameplayStatics.GetGameMode`)))
  (set `self.BPREF_Gamemode` _asbp_rektgame_mode)
  (bind _outactors (`GameplayStatics.GetAllActorsOfClass` "/Game/Blueprints/Checkpoints/BP_Tracker.BP_Tracker_C"))
  (set `self.BPREF_Tracker` (`|GetArrayItem` _outactors))
  (`self.SetDynamicMaterialsInstances`)
  (`self.SetInitialValuesOfDMI`)
  (`SceneComponent.SetVisibility` (`/Game/Blueprints/Checkpoints/BP_Checkpoint.FinishLine_Plane` (`/Game/Blueprints/Checkpoints/BP_Tracker.StartingLine` (`self.BPREF_Tracker`))) true false)
  (bind _outactors_2 (`GameplayStatics.GetAllActorsOfClass` "/Game/Blueprints/AI/BP_MasterEnemy.BP_MasterEnemy_C"))
  (for _ _outactors_2
    (set `self.NumberOfStartingEnemies` (+ (`self.NumberOfStartingEnemies`) 1))))

(event `EVNT_Crossed`
  (bind _bpref_mastervehicle (`self.BPREF_MasterVehicle`))
  (bind (_returnvalue_location _returnvalue_rotation) (`KismetMathLibrary.BreakTransform` (`SceneComponent.K2_GetComponentToWorld` (`self.Arrow`))))
  ;[1 1 1] Changes things here
  (if (`self.ActorHasTag` (`self.CrossingActor`) "Vehicle")
    (set `/Game/Vehicles/MasterVehicle/BP_MasterVehicle.LastCrossedCheckpoint` (`self.CheckpointNumber`) _bpref_mastervehicle)
    (set `/Game/Vehicles/MasterVehicle/BP_MasterVehicle.TotalCrossedCheckpoints` (+ (`/Game/Vehicles/MasterVehicle/BP_MasterVehicle.TotalCrossedCheckpoints` _bpref_mastervehicle) 1) _bpref_mastervehicle)
    (set `/Game/Vehicles/MasterVehicle/BP_MasterVehicle.Respawn` (`KismetMathLibrary.MakeTransform` _returnvalue_location _returnvalue_rotation) (`self.BPREF_MasterVehicle`))
    (`LightComponent.SetLightColor` (`self.RectLight`) (struct :`G` 1.0 :`B` 1.0 :`A` 1.0) true)
    (`AkGameplayStatics.PostEventAtLocation` "/Game/Audio/AKEvents/UI/Play_UI_Babypark_Checkpoint.Play_UI_Babypark_Checkpoint")
    (`/Game/Vehicles/MasterVehicle/BP_MasterVehicle.EVNT_BoostRefill` (`self.BPREF_MasterVehicle`))))

(event `EVNT_LapFinished`
  (bind _bpref_mastervehicle (`self.BPREF_MasterVehicle`))
  (bind _bpref_mastervehicle_2 (`self.BPREF_MasterVehicle`))
  (bind _bpref_tracker (`self.BPREF_Tracker`))
  (bind _w_lapdisplayer (`/Game/Widgets/InGame/W_Main.W_LapDisplayer` (`/Game/Blueprints/Base/BP_REKTGameMode.WREF_Main` (`self.BPREF_Gamemode`))))
  ;[1 1 1] Changes things here
  (set `/Game/Blueprints/Checkpoints/BP_Tracker.LapsDone` (+ (`/Game/Blueprints/Checkpoints/BP_Tracker.LapsDone` _bpref_tracker) 1) _bpref_tracker)
  (`self.SetTime`)
  (set `/Game/Vehicles/MasterVehicle/BP_MasterVehicle.LastCrossedCheckpoint` 0 _bpref_mastervehicle_2)
  (set `/Game/Vehicles/MasterVehicle/BP_MasterVehicle.TotalCrossedCheckpoints` 0 _bpref_mastervehicle_2)
  (bind _outactors (`GameplayStatics.GetAllActorsOfClass` "BP_Checkpoint_C"))
  (for _array_element _outactors
    (bind _dmi_leftpillar (`/Game/Blueprints/Checkpoints/BP_Checkpoint.DMI_LeftPillar` _array_element))
    (`MaterialInstanceDynamic.SetVectorParameterValue` _dmi_leftpillar "Base" (struct :`R` 1.0 :`B` 0.846873))
    (`MaterialInstanceDynamic.SetVectorParameterValue` (`/Game/Blueprints/Checkpoints/BP_Checkpoint.DMI_RightPillar` _array_element) "Base" (struct :`R` 1.0 :`B` 0.846873))
    (`MaterialInstanceDynamic.SetVectorParameterValue` _dmi_leftpillar "Tint" (struct :`R` 0.775822 :`B` 0.53948))
    (`MaterialInstanceDynamic.SetVectorParameterValue` (`/Game/Blueprints/Checkpoints/BP_Checkpoint.DMI_RightPillar` _array_element) "Tint" (struct :`R` 0.775822 :`B` 0.53948))
    (`LightComponent.SetLightColor` (`/Game/Blueprints/Checkpoints/BP_Checkpoint.RectLight` _array_element) (struct :`R` 1.0 :`B` 1.0 :`A` 1.0) true)
    (set `/Game/Vehicles/MasterVehicle/BP_MasterVehicle.Charge` 3 _bpref_mastervehicle)
    (`Widget.SetVisibility` _w_lapdisplayer "Visible")
    (`TextBlock.SetText` (`/Game/Widgets/InGame/W_LapDisplayer.TextBlock_laps` _w_lapdisplayer) (`|FormatText` "Lap {Lap}" (+ (`/Game/Blueprints/Checkpoints/BP_Tracker.LapsDone` (`self.BPREF_Tracker`)) 1)))
    (`UserWidget.PlayAnimation` _w_lapdisplayer (`/Game/Widgets/InGame/W_LapDisplayer.Appearance` _w_lapdisplayer) 0.0 1 "Forward" 1.0)
    (`AkGameplayStatics.PostEvent` "/Game/Audio/AKEvents/UI/Play_UI_Lap_Finish.Play_UI_Lap_Finish" _bpref_mastervehicle)
    (`KismetSystemLibrary.Delay` 2.0)
    (`Widget.SetVisibility` _w_lapdisplayer "Hidden")))

(event `EVNT_EndRace`
  (bind _finalscore (`self.FinalScore`))
  (bind _bpref_mastervehicle (`self.BPREF_MasterVehicle`))
  (bind _medalsscores (`/Game/Blueprints/Checkpoints/BP_Tracker.MedalsScores` (`self.BPREF_Tracker`)))
  (bind (_returnvalue_days _returnvalue_hours _returnvalue_minutes _returnvalue_seconds _returnvalue_milliseconds) (`KismetMathLibrary.BreakTimespan` (`KismetMathLibrary.FromMilliseconds` (`/Game/Vehicles/MasterVehicle/BP_MasterVehicle.Timer` (`self.BPREF_MasterVehicle`)))))
  (bind _output (`|GetArrayItem` _medalsscores))
  ;[1 1 1] Changes things here
  (`WidgetLayoutLibrary.RemoveAllWidgets`)
  (`self.DisableInput` _bpref_mastervehicle (`GameplayStatics.GetPlayerController` 0))
  (`/Game/Vehicles/MasterVehicle/BP_MasterVehicle.SetBrakeInput` _bpref_mastervehicle 1.0 false)
  (bind _returnvalue (`|CreateWidget` "/Game/Widgets/EndRace/W_FadeToBlack.W_FadeToBlack_C"))
  (`UserWidget.AddToViewport` _returnvalue 0)
  (bind (_direction _faderalpha) (`Timeline|SetAlphaFader`)
    (:`Update`
      (`Image.SetColorAndOpacity` (`/Game/Widgets/EndRace/W_FadeToBlack.Image_Fader` _returnvalue) (make `LinearColor` 0.0 0.0 0.0 _faderalpha)))
    (:`Finished`
      (`GameplayStatics.SetGamePaused` true)
      (`self.SetFastestLap`)
      (`self.DisableInput` (`GameplayStatics.GetPlayerPawn` 0) null)
      (`WidgetLayoutLibrary.RemoveAllWidgets`)
      (bind _returnvalue_2 (`|CreateWidget` "/Game/Widgets/EndRace/W_EndRace.W_EndRace_C"))
      (set `self.WREF_EndRace` _returnvalue_2)
      (set `/Game/Widgets/EndRace/W_EndRaceDataRow.Data` (`|FormatText` "{Minutes}:{Seconds}.{Milliseconds}" (`KismetTextLibrary.Conv_IntToText` _returnvalue_minutes false true 2) (`KismetTextLibrary.Conv_IntToText` _returnvalue_seconds false true 2) (`KismetTextLibrary.Conv_IntToText` _returnvalue_milliseconds false true 3)) (`/Game/Widgets/EndRace/W_EndRace.W_EndRaceDataTime` (`self.WREF_EndRace`)))
      (bind _outactors (`GameplayStatics.GetAllActorsOfClass` "/Game/Blueprints/Equipements/Turrets/BP_MasterTurret.BP_MasterTurret_C"))
      (for _ _outactors
        (set `self.TurretsDeployed` (+ (`self.TurretsDeployed`) 1)))
      (set `/Game/Widgets/EndRace/W_EndRaceDataRow.Data` (`KismetTextLibrary.Conv_IntToText` (`self.TurretsDeployed`)) (`/Game/Widgets/EndRace/W_EndRace.W_EndRaceDataTurrets` (`self.WREF_EndRace`)))
      (set `/Game/Widgets/EndRace/W_EndRaceDataRow.Data` (`KismetTextLibrary.Conv_IntToText` (`/Game/Vehicles/MasterVehicle/BP_MasterVehicle.PlacedTraps` (`self.BPREF_MasterVehicle`))) (`/Game/Widgets/EndRace/W_EndRace.W_EndRaceDataTraps` (`self.WREF_EndRace`)))
      (set `/Game/Widgets/EndRace/W_EndRaceDataRow.Data` (`KismetTextLibrary.Conv_IntToText` (`/Game/Vehicles/MasterVehicle/BP_MasterVehicle.Currency` (`self.BPREF_MasterVehicle`))) (`/Game/Widgets/EndRace/W_EndRace.W_EndRaceDataCurrency` (`self.WREF_EndRace`)))
      (set `/Game/Widgets/EndRace/W_EndRaceDataRow.Data` (`KismetTextLibrary.Conv_IntToText` (`self.FinishingEnemies`)) (`/Game/Widgets/EndRace/W_EndRace.W_EndRaceDataFinishers` (`self.WREF_EndRace`)))
      (set `/Game/Widgets/EndRace/W_EndRaceDataRow.Data` (`KismetTextLibrary.Conv_IntToText` (`/Game/Vehicles/MasterVehicle/BP_MasterVehicle.EnemiesKilled` (`self.BPREF_MasterVehicle`))) (`/Game/Widgets/EndRace/W_EndRace.W_EndRaceDataKilledEnemies` (`self.WREF_EndRace`)))
      (`self.SetFinalScore`)
      (if (<= _finalscore 0)
        (`Image.SetBrushFromTexture` (`/Game/Widgets/EndRace/W_EndRace.Image_Medal` (`self.WREF_EndRace`)) "/Game/Widgets/Ressources/EndRace/Medals/UI_03_BronzeMedal.UI_03_BronzeMedal" false)
        (`TextBlock.SetText` (`/Game/Widgets/EndRace/W_EndRace.TextBlock_Score` (`self.WREF_EndRace`)) (`KismetTextLibrary.Conv_IntToText` (`self.FinalScore`)) :!label _label)
        (`UserWidget.AddToViewport` (`self.WREF_EndRace`) 0)
        (`self.EnableInput` (`GameplayStatics.GetPlayerController` 0))
        (bind _returnvalue_3 (`GameplayStatics.CreateSaveGameObject` "/Game/BP_SaveGame.BP_SaveGame_C"))
        (set `self.SAVEREF_RaceInformations` _returnvalue_3)
        (`self.SetBestScore`)
        (set `/Game/BP_SaveGame.Time` (`/Game/Vehicles/MasterVehicle/BP_MasterVehicle.Timer` (`self.BPREF_MasterVehicle`)) (`self.SAVEREF_RaceInformations`))
        (`self.SetNumberOfMedals`)
        (`self.SetBestTime`)
        (bind _returnvalue_4 (`GameplayStatics.GetCurrentLevelName` true))
        (`GameplayStatics.SaveGameToSlot` (`self.SAVEREF_RaceInformations`) (`KismetStringLibrary.Concat_StrStr` _returnvalue_4 "_SaveSlot"))
        (elif (and (>= _finalscore (`|GetArrayItem` _medalsscores 1)) (< _finalscore _output))
          (`Image.SetBrushFromTexture` (`/Game/Widgets/EndRace/W_EndRace.Image_Medal` (`self.WREF_EndRace`)) "/Game/Widgets/Ressources/EndRace/Medals/UI_02_SilverMedal.UI_02_SilverMedal" false)
          (goto _label)
          (elif (>= _finalscore _output)
            (`Image.SetBrushFromTexture` (`/Game/Widgets/EndRace/W_EndRace.Image_Medal` (`self.WREF_EndRace`)) "/Game/Widgets/Ressources/EndRace/Medals/UI_01_GoldMedal.UI_01_GoldMedal" false)
            (goto _label)))))))

(event `Key|AnyKey` :paused true
  (params (Key :type "Key Structure"))
  (:`Pressed`
    (if (`/Game/Widgets/EndRace/W_EndRace.bCanEnterMenu` (`self.WREF_EndRace`))
      (`GameplayStatics.OpenLevel` "Menu_Persistent"))))

(event `self.Trigger.OnComponentBeginOverlap`
  (params (OverlappedComponent :type "PrimitiveComponent Object Reference") (OtherActor :type "Actor Object Reference") (OtherComp :type "PrimitiveComponent Object Reference") (OtherBodyIndex :type Integer) (bFromSweep :type Boolean) (SweepResult :type "HitResult Structure (by ref)"))
  (if (`self.ActorHasTag` OtherActor "Vehicle")
    (if (`self.CheckDirection`)
      (`MaterialInstanceDynamic.SetVectorParameterValue` (`self.DMI_RightPillar`) "Base" (struct :`R` 0.099899 :`G` 0.502887 :`B` 1.0))
      (`MaterialInstanceDynamic.SetVectorParameterValue` (`self.DMI_LeftPillar`) "Base" (struct :`R` 0.099899 :`G` 0.502887 :`B` 1.0))
      (`MaterialInstanceDynamic.SetVectorParameterValue` (`self.DMI_RightPillar`) "Tint" (struct :`R` 0.009721 :`G` 0.351533 :`B` 0.376262))
      (`MaterialInstanceDynamic.SetVectorParameterValue` (`self.DMI_LeftPillar`) "Tint" (struct :`R` 0.009721 :`G` 0.351533 :`B` 0.376262)))))

(event `self.Trigger.OnComponentEndOverlap`
  (params (OverlappedComponent :type "PrimitiveComponent Object Reference") (OtherActor :type "Actor Object Reference") (OtherComp :type "PrimitiveComponent Object Reference") (OtherBodyIndex :type Integer))
  (bind _bpref_tracker (`self.BPREF_Tracker`))
  (bind _bpref_mastervehicle (`self.BPREF_MasterVehicle`))
  ;[1 0 0] /!\ DO NOT TOUCH /!\
  ;;[1 1 1] Check crossing direction
  (set `self.CrossingActor` OtherActor)
  (if (and (`self.ActorHasTag` (`self.CrossingActor`) "Enemy") (== (`self.CheckpointNumber`) 0))
    (bind _asbp_master_enemy (cast `/Game/Blueprints/AI/BP_MasterEnemy` (`self.CrossingActor`)))
    (set `self.BPREF_MasterEnemy` _asbp_master_enemy)
    (set `/Game/Vehicles/MasterVehicle/BP_MasterVehicle.Score` (- (`/Game/Vehicles/MasterVehicle/BP_MasterVehicle.Score` _bpref_mastervehicle) 100) _bpref_mastervehicle)
    (set `self.FinishingEnemies` (+ (`self.FinishingEnemies`) 1))
    (elif (`self.CheckDirection`)
      (`self.EVNT_Crossed`)
      ;;[1 1 1] Check if last checkpoint
      (if (and (== (`/Game/Vehicles/MasterVehicle/BP_MasterVehicle.LastCrossedCheckpoint` (`self.BPREF_MasterVehicle`)) 0) (>= (`/Game/Vehicles/MasterVehicle/BP_MasterVehicle.TotalCrossedCheckpoints` (`self.BPREF_MasterVehicle`)) (`/Game/Blueprints/Checkpoints/BP_Tracker.NumberOfCheckpoints` (`self.BPREF_Tracker`))))
        (`self.EVNT_LapFinished`)
        (if (== (`/Game/Blueprints/Checkpoints/BP_Tracker.LapsDone` _bpref_tracker) (`/Game/Blueprints/Checkpoints/BP_Tracker.Laps` _bpref_tracker))
          (`self.EVNT_EndRace`))))))

(fn `AddCurrencyToScore`
  (bind _bpref_mastervehicle (`self.BPREF_MasterVehicle`))
  (set `/Game/Vehicles/MasterVehicle/BP_MasterVehicle.Score` (+ (`/Game/Vehicles/MasterVehicle/BP_MasterVehicle.Score` _bpref_mastervehicle) 1) _bpref_mastervehicle))

(fn `SetBestScore`
  (if (>= (`self.FinalScore`) (`/Game/BP_SaveGame.BestScore` (`self.SAVEREF_RaceInformations`)))
    (set `/Game/BP_SaveGame.BestScore` (`self.FinalScore`) (`self.SAVEREF_RaceInformations`)))
  (return))

(fn `SetBestTime`
  (if (<= (`/Game/Vehicles/MasterVehicle/BP_MasterVehicle.Timer` (`self.BPREF_MasterVehicle`)) (`/Game/BP_SaveGame.BestTime` (`self.SAVEREF_RaceInformations`)))
    (set `/Game/BP_SaveGame.BestTime` (`/Game/Vehicles/MasterVehicle/BP_MasterVehicle.Timer` (`self.BPREF_MasterVehicle`)) (`self.SAVEREF_RaceInformations`)))
  (return))

(fn `SetDynamicMaterialsInstances`
  (bind _returnvalue (`PrimitiveComponent.CreateDynamicMaterialInstance` (`self.Pillar_Right`) 2 "/Game/Materials/M_CheckPoint/MI_Checkpoint_Grid.MI_Checkpoint_Grid" "None"))
  (set `self.DMI_RightPillar` _returnvalue)
  (bind _returnvalue_2 (`PrimitiveComponent.CreateDynamicMaterialInstance` (`self.Pillar_Left`) 2 "/Game/Materials/M_CheckPoint/MI_Checkpoint_Grid.MI_Checkpoint_Grid" "None"))
  (set `self.DMI_LeftPillar` _returnvalue_2))

(fn `SetFastestLap`
  (bind _bpref_mastervehicle (`self.BPREF_MasterVehicle`))
  (for _array_element (`/Game/Vehicles/MasterVehicle/BP_MasterVehicle.lapsTimes` (`self.BPREF_MasterVehicle`))
    (if (> (`/Game/Vehicles/MasterVehicle/BP_MasterVehicle.LapTime` _bpref_mastervehicle) _array_element)
      (set `/Game/Vehicles/MasterVehicle/BP_MasterVehicle.LapTime` _array_element _bpref_mastervehicle)))
  (return))

(fn `SetFinalScore`
  (bind _times (`/Game/Blueprints/Checkpoints/BP_Tracker.Times` (`self.BPREF_Tracker`)))
  (bind _returnvalue (/ (`/Game/Vehicles/MasterVehicle/BP_MasterVehicle.Timer` (`self.BPREF_MasterVehicle`)) 1000.0))
  (if (<= _returnvalue (`|GetArrayItem` _times))
    (bind _output_get (`self.SetScoreDependingOnFinishedTime` 0))
    (set `self.FinalScore` _output_get)
    (`self.GetTimeScore` 0)
    (elif (<= _returnvalue (`|GetArrayItem` _times 1))
      (bind _output_get_2 (`self.SetScoreDependingOnFinishedTime` 1))
      (set `self.FinalScore` _output_get_2)
      (`self.GetTimeScore` 1)
      (elif (<= _returnvalue (`|GetArrayItem` _times 2))
        (bind _output_get_3 (`self.SetScoreDependingOnFinishedTime` 2))
        (set `self.FinalScore` _output_get_3)
        (`self.GetTimeScore` 2)
        (elif (<= _returnvalue (`|GetArrayItem` _times 3))
          (bind _output_get_4 (`self.SetScoreDependingOnFinishedTime` 3))
          (set `self.FinalScore` _output_get_4)
          (`self.GetTimeScore` 3)
          (elif (<= _returnvalue (`|GetArrayItem` _times 3))
            (bind _output_get_5 (`self.SetScoreDependingOnFinishedTime` 4))
            (set `self.FinalScore` _output_get_5)
            (`self.GetTimeScore` 4))))))
  (return))

(fn `SetInitialValuesOfDMI`
  (`MaterialInstanceDynamic.SetVectorParameterValue` (`self.DMI_RightPillar`) "Base" (struct :`R` 1.0 :`B` 0.846873))
  (`MaterialInstanceDynamic.SetVectorParameterValue` (`self.DMI_LeftPillar`) "Base" (struct :`R` 1.0 :`B` 0.846873))
  (`MaterialInstanceDynamic.SetVectorParameterValue` (`self.DMI_RightPillar`) "Tint" (struct :`R` 0.775822 :`B` 0.53948))
  (`MaterialInstanceDynamic.SetVectorParameterValue` (`self.DMI_LeftPillar`) "Tint" (struct :`R` 0.775822 :`B` 0.53948)))

(fn `SetNumberOfMedals`
  (bind _finalscore (`self.FinalScore`))
  (bind _medalsscores (`/Game/Blueprints/Checkpoints/BP_Tracker.MedalsScores` (`self.BPREF_Tracker`)))
  (bind _output (`|GetArrayItem` _medalsscores))
  (if (<= _finalscore 0)
    (set `/Game/BP_SaveGame.Medals` 1 (`self.SAVEREF_RaceInformations`))
    (elif (and (>= _finalscore (`|GetArrayItem` _medalsscores 1)) (< _finalscore _output))
      (set `/Game/BP_SaveGame.Medals` 2 (`self.SAVEREF_RaceInformations`))
      (elif (>= _finalscore _output)
        (set `/Game/BP_SaveGame.Medals` 3 (`self.SAVEREF_RaceInformations`)))))
  (return))

(fn `SetTime`
  (bind _bpref_mastervehicle (`self.BPREF_MasterVehicle`))
  (bind _output_get (set `/Game/Vehicles/MasterVehicle/BP_MasterVehicle.LapTime` (`/Game/Vehicles/MasterVehicle/BP_MasterVehicle.Timer` _bpref_mastervehicle) _bpref_mastervehicle))
  (`KismetArrayLibrary.Array_Add` (`/Game/Vehicles/MasterVehicle/BP_MasterVehicle.lapsTimes` _bpref_mastervehicle) _output_get))

(fn `UserConstructionScript`)