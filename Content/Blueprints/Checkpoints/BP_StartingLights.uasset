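; Race starting lights actor that runs the start countdown on BeginPlay and releases the player's vehicle.
; It adds the W_StartupCount widget and creates a dynamic material instance for each of four light rows.
; SetLights lights rows in sequence, then switches their color after a randomized delay for an unpredictable start.
; It then calls EVNTPossess on the player's BP_MasterVehicle and turns the lights off a few seconds later.
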(event `self.ReceiveBeginPlay`
  (bind _returnvalue (`|CreateWidget` "/Game/Widgets/W_StartupCount.W_StartupCount_C"))
  (`UserWidget.AddToViewport` _returnvalue 0)
  (`self.SetDynamicMaterialsInstances`)
  (`MaterialInstanceDynamic.SetScalarParameterValue` (`self.DMI_Row1`) "isLit?" 1.0)
  (`KismetSystemLibrary.Delay` 1.0)
  (`MaterialInstanceDynamic.SetScalarParameterValue` (`self.DMI_Row2`) "isLit?" 1.0)
  (`KismetSystemLibrary.Delay` 1.0)
  (`MaterialInstanceDynamic.SetScalarParameterValue` (`self.DMI_Row3`) "isLit?" 1.0)
  (`KismetSystemLibrary.Delay` 1.0)
  (`MaterialInstanceDynamic.SetScalarParameterValue` (`self.DMI_Row4`) "isLit?" 1.0)
  (`KismetSystemLibrary.Delay` (`KismetMathLibrary.RandomFloatInRange` 0.7 1.3))
  (`MaterialInstanceDynamic.SetVectorParameterValue` (`self.DMI_Row1`) "Color" (struct :`G` 1.0 :`B` 1.0 :`A` 1.0))
  (`MaterialInstanceDynamic.SetVectorParameterValue` (`self.DMI_Row2`) "Color" (struct :`G` 1.0 :`B` 1.0 :`A` 1.0))
  (`MaterialInstanceDynamic.SetVectorParameterValue` (`self.DMI_Row3`) "Color" (struct :`G` 1.0 :`B` 1.0 :`A` 1.0))
  (`MaterialInstanceDynamic.SetVectorParameterValue` (`self.DMI_Row4`) "Color" (struct :`G` 1.0 :`B` 1.0 :`A` 1.0))
  (bind _asbp_master_vehicle (cast `/Game/Vehicles/MasterVehicle/BP_MasterVehicle` (`GameplayStatics.GetPlayerPawn` 0)))
  (`/Game/Vehicles/MasterVehicle/BP_MasterVehicle.EVNT_Possess` _asbp_master_vehicle)
  (`KismetSystemLibrary.Delay` 5.0)
  (`MaterialInstanceDynamic.SetScalarParameterValue` (`self.DMI_Row1`) "isLit?" 0.0)
  (`MaterialInstanceDynamic.SetScalarParameterValue` (`self.DMI_Row2`) "isLit?" 0.0)
  (`MaterialInstanceDynamic.SetScalarParameterValue` (`self.DMI_Row3`) "isLit?" 0.0)
  (`MaterialInstanceDynamic.SetScalarParameterValue` (`self.DMI_Row4`) "isLit?" 0.0))

(fn `SetDynamicMaterialsInstances`
  (bind _returnvalue (`PrimitiveComponent.CreateDynamicMaterialInstance` (`self.StartingLights`) 4 "/Game/Materials/Props/M_StartingLights.M_StartingLights" "None"))
  (set `self.DMI_Row1` _returnvalue)
  (bind _returnvalue_2 (`PrimitiveComponent.CreateDynamicMaterialInstance` (`self.StartingLights`) 3 "/Game/Materials/Props/M_StartingLights.M_StartingLights" "None"))
  (set `self.DMI_Row2` _returnvalue_2)
  (bind _returnvalue_3 (`PrimitiveComponent.CreateDynamicMaterialInstance` (`self.StartingLights`) 2 "/Game/Materials/Props/M_StartingLights.M_StartingLights" "None"))
  (set `self.DMI_Row3` _returnvalue_3)
  (bind _returnvalue_4 (`PrimitiveComponent.CreateDynamicMaterialInstance` (`self.StartingLights`) 1 "/Game/Materials/Props/M_StartingLights.M_StartingLights" "None"))
  (set `self.DMI_Row4` _returnvalue_4))

(fn `UserConstructionScript`)