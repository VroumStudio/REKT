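; Heat map actor that records where a tracked player moves over its plane and can export the result as an image.
; Each tick it traces down from PlayerRef and, on hitting itself, draws a heat splat material at the plane-local position into a runtime render target cleared at BeginPlay.
; PrintHeatMAP draws the floor heat map material into a bake target and, once, optionally exports it as a timestamped PNG.
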(event `self.ReceiveBeginPlay`
  (set `self.BPREF_MasterVehicle` (`GameplayStatics.GetPlayerPawn` 0))
  (`KismetRenderingLibrary.ClearRenderTarget2D` (`self.RenderTargetRuntime`)))

(event `self.ReceiveTick`
  (params (DeltaSeconds :type "Float (single-precision)"))
  (bind _playerref (`self.PlayerRef`))
  (bind _returnvalue (`self.K2_GetActorLocation` _playerref))
  (bind (_returnvalue_x _returnvalue_y _returnvalue_z) (`KismetMathLibrary.BreakVector` (`SceneComponent.K2_GetComponentLocation` (`self.NewPlane`))))
  (`/Engine/EditorBlueprintResources/StandardMacros.IsValid` _playerref
    (:`Is Valid`
      (bind _outhits (`KismetSystemLibrary.LineTraceMultiForObjects` :`Start` _returnvalue :`End` (`KismetMathLibrary.MakeVector` (.x _returnvalue) (.y _returnvalue) (- _returnvalue_z 1.0)) :`ObjectTypes` (`|MakeArray` "ObjectTypeQuery1" "ObjectTypeQuery2" :!type "EObjectTypeQuery Enum") :`bIgnoreSelf` false))
      (for _array_element _outhits
        (bind (_bblockinghit _binitialoverlap _time _distance _location _impactpoint _normal _impactnormal _physmat _hitactor) (`GameplayStatics.BreakHitResult` _array_element))
        (if (and _bblockinghit (== _hitactor self))
          (`self.DrawToRenderTarget` _location (`self.Strengh`) (`self.Size`)))))))

(event `DrawToRenderTarget`
  (params (Location :type "Vector Structure") (Strengh :type "Float (double-precision)") (Size :type "Float (double-precision)"))
  (bind _mid_heatsplat (`self.MID_HeatSplat`))
  (`MaterialInstanceDynamic.SetScalarParameterValue` _mid_heatsplat "Size" Size)
  (`MaterialInstanceDynamic.SetScalarParameterValue` _mid_heatsplat "Strengh" Strengh)
  (`MaterialInstanceDynamic.SetVectorParameterValue` _mid_heatsplat "Position" (`KismetMathLibrary.Conv_VectorToLinearColor` (/ (`KismetMathLibrary.TransformLocation` (`KismetMathLibrary.InvertTransform` (`SceneComponent.K2_GetComponentToWorld` (`self.NewPlane`))) Location) (`self.Resolution`))))
  (`KismetRenderingLibrary.DrawMaterialToRenderTarget` (`self.RenderTargetRuntime`) _mid_heatsplat))

(event `PrintHeatMAP`
  (bind _rendertargetbake (`self.RenderTargetBake`))
  (bind (_year _month _day _hour _minute _second) (`KismetMathLibrary.BreakDateTime` (`KismetMathLibrary.Now`)))
  ;[1 1 1] Export HeatMAP
  (`KismetRenderingLibrary.DrawMaterialToRenderTarget` _rendertargetbake "/Game/Steve_HeatMAP/Material/M_FloorHeatMap.M_FloorHeatMap")
  (`/Engine/EditorBlueprintResources/StandardMacros.DoOnce` false
    (:`Completed`
      (if (`self.Export HeatMap ?`)
        (`KismetRenderingLibrary.ExportRenderTarget` _rendertargetbake (`KismetStringLibrary.Concat_StrStr` (`self.Export path`) (`self.FolderName`)) (`KismetStringLibrary.Concat_StrStr` (`self.HeatMap File Name`) (`KismetStringLibrary.Conv_IntToString` _day) "-" (`KismetStringLibrary.Conv_IntToString` _month) "_" (`KismetStringLibrary.Conv_IntToString` _hour) "H" (`KismetStringLibrary.Conv_IntToString` _minute) "_" (`KismetStringLibrary.Conv_IntToString` _second) ".png"))))))

(fn `UserConstructionScript`
  (bind _returnvalue (`KismetMaterialLibrary.CreateDynamicMaterialInstance` "/Game/Steve_HeatMAP/Material/M_HeatSplat.M_HeatSplat"))
  (set `self.MID_HeatSplat` _returnvalue))