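; BP_Mine_Trap is a mine trap that pulses a warning glow and animates when something overlaps its collision box.
; On BeginPlay it creates a dynamic emissive material, caches its Anim Blueprint and plays the Opacity_Warning timeline to drive the glow's opacity.
; Any overlap sets IsTriggered on the Anim Blueprint and holds full opacity briefly, then resets both and restarts the timeline.
; Tick prints the trigger state for debugging.
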(event `self.ReceiveTick`
  (params (DeltaSeconds :type "Float (single-precision)"))
  (`KismetSystemLibrary.PrintString` (`KismetStringLibrary.Concat_StrStr` "Is Triggered ? " (`KismetStringLibrary.Conv_BoolToString` (`/Game/Traps/Mine_trap/Mine_Trap_Anim_BP.Is Triggered` (`self.MineTrap_Anim_BP`)))) true true (struct :`R` 1.0 :`A` 1.0) 0.0))

(event `self.ReceiveBeginPlay`
  (bind _returnvalue (`PrimitiveComponent.CreateDynamicMaterialInstance` (`self.Mine_Trap_LOW_Rigged`) 1 "/Game/Traps/Mine_trap/M_Emissive_Mine_Trap_Instance.M_Emissive_Mine_Trap_Instance" "None"))
  (set `self.Mine_Emissive_Instance` _returnvalue)
  (bind _asmine_trap_anim_bp (cast `/Game/Traps/Mine_trap/Mine_Trap_Anim_BP` (`SkeletalMeshComponent.GetAnimInstance` (`self.Mine_Trap_LOW_Rigged`))))
  (set `self.MineTrap_Anim_BP` _asmine_trap_anim_bp)
  (bind (_direction _opacity_track) (`Timeline|Opacity_Warning` :!label _label)
    (:`Update`
      (`MaterialInstanceDynamic.SetScalarParameterValue` (`self.Mine_Emissive_Instance`) "Opacity" _opacity_track))))

(event `self.Collision_Box.OnComponentBeginOverlap`
  (params (OverlappedComponent :type "PrimitiveComponent Object Reference") (OtherActor :type "Actor Object Reference") (OtherComp :type "PrimitiveComponent Object Reference") (OtherBodyIndex :type Integer) (bFromSweep :type Boolean) (SweepResult :type "HitResult Structure (by ref)"))
  (set `/Game/Traps/Mine_trap/Mine_Trap_Anim_BP.Is Triggered` true (`self.MineTrap_Anim_BP`))
  (`|ExecutionSequence`
    (:`then_0`
      (goto _label :!via `Stop`))
    (:`then_1`
      (`MaterialInstanceDynamic.SetScalarParameterValue` (`self.Mine_Emissive_Instance`) "Opacity" 1.0)
      (`KismetSystemLibrary.Delay` 2.0)
      (`MaterialInstanceDynamic.SetScalarParameterValue` (`self.Mine_Emissive_Instance`) "Opacity" 0.0)
      (set `/Game/Traps/Mine_trap/Mine_Trap_Anim_BP.Is Triggered` false (`self.MineTrap_Anim_BP`))
      (goto _label :!via `PlayFromStart`))))

(event `self.Collision_Box.OnComponentEndOverlap`
  (params (OverlappedComponent :type "PrimitiveComponent Object Reference") (OtherActor :type "Actor Object Reference") (OtherComp :type "PrimitiveComponent Object Reference") (OtherBodyIndex :type Integer)))

(fn `UserConstructionScript`)