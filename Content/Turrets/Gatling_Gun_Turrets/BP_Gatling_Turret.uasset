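; Gatling gun turret actor that targets whatever actor enters its trigger box.
; Box overlaps toggle CanShoot on the turret's animation Blueprint, which also receives the overlapping actor's lowered position as its aim Location.
; While active, Tick uses a short Delay to pace debug-drawn visibility traces toward the target and spawns a hit explosion emitter at each trace location, without applying damage.
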(event `self.ReceiveBeginPlay`
  (bind _asturret_anim_bp (cast `/Game/Turrets/Gatling_Gun_Turrets/Animation/Turret_Anim_BP` (`SkeletalMeshComponent.GetAnimInstance` (`self.Gatling_Turret_LOW_Rigged`))))
  (set `self.Turret_Anim_BP` _asturret_anim_bp))

(event `self.ReceiveTick`
  (params (DeltaSeconds :type "Float (single-precision)"))
  (if (`/Game/Turrets/Gatling_Gun_Turrets/Animation/Turret_Anim_BP.Can_Shoot` (`self.Turret_Anim_BP`))
    (bind _returnvalue (`self.K2_GetActorLocation` (stale `self.Box.OnComponentBeginOverlap` OtherActor)))
    (set `/Game/Turrets/Gatling_Gun_Turrets/Animation/Turret_Anim_BP.Location` (- _returnvalue (0.0 0.0 200.0)) (`self.Turret_Anim_BP`))
    (`KismetSystemLibrary.Delay` 0.1)
    (bind _outhit (`KismetSystemLibrary.LineTraceSingle` :`Start` (+ (`SceneComponent.K2_GetComponentLocation` (`self.Gatling_Turret_LOW_Rigged`)) (0.0 0.0 300.0)) :`End` (- _returnvalue (0.0 0.0 100.0)) :`TraceChannel` "TraceTypeQuery1" :`DrawDebugType` "ForOneFrame"))
    (`GameplayStatics.SpawnEmitterAtLocation` "/Game/Turrets/Gatling_Gun_Turrets/FX/PS_Explosion_HIT_Gatling.PS_Explosion_HIT_Gatling" (`.Location` (`GameplayStatics.BreakHitResult` _outhit)))))

(event `self.Box.OnComponentBeginOverlap`
  (params (OverlappedComponent :type "PrimitiveComponent Object Reference") (OtherActor :type "Actor Object Reference") (OtherComp :type "PrimitiveComponent Object Reference") (OtherBodyIndex :type Integer) (bFromSweep :type Boolean) (SweepResult :type "HitResult Structure (by ref)"))
  (set `/Game/Turrets/Gatling_Gun_Turrets/Animation/Turret_Anim_BP.Can_Shoot` true (`self.Turret_Anim_BP`)))

(event `self.Box.OnComponentEndOverlap`
  (params (OverlappedComponent :type "PrimitiveComponent Object Reference") (OtherActor :type "Actor Object Reference") (OtherComp :type "PrimitiveComponent Object Reference") (OtherBodyIndex :type Integer))
  (set `/Game/Turrets/Gatling_Gun_Turrets/Animation/Turret_Anim_BP.Can_Shoot` false (`self.Turret_Anim_BP`)))

(fn `UserConstructionScript`)