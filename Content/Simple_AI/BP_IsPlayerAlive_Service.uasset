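; Behavior tree service for the simple AI that tracks whether the player is alive and where they are.
; On tick it treats a valid pawn controlled by player controller 0 as alive and writes that result to the IsPlayerAlive blackboard key.
; It also writes the pawn's location to PlayerObject as a vector, or the zero vector when no valid pawn exists.
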(event `self.ReceiveTick`
  (params (OwnerActor :type "Actor Object Reference") (DeltaSeconds :type "Float (single-precision)"))
  (bind _returnvalue (`KismetSystemLibrary.IsValid` (`Controller.K2_GetPawn` (`GameplayStatics.GetPlayerController` 0))))
  (`BTFunctionLibrary.SetBlackboardValueAsBool` (`self.IsPlayerAlive`) _returnvalue)
  (if _returnvalue
    (`BTFunctionLibrary.SetBlackboardValueAsVector` (`self.PlayerObject`) (`Actor.K2_GetActorLocation` (`Controller.K2_GetPawn` (`GameplayStatics.GetPlayerController` 0))))
    (else
      (`BTFunctionLibrary.SetBlackboardValueAsVector` (`self.PlayerObject`)))))